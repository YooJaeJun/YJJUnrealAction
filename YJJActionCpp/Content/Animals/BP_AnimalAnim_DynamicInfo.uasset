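; Animation info actor that gathers movement state for an animal character and exposes state-transition checks for moving, rotating, jumping and falling.
; Tick_Info caches the owner as BP_Character, then derives speed, movement direction, control-versus-body turn values and falling state, destroying itself if the owner is invalid.
; It copies foot, hand, pelvis and ground-slope data from FeetComponent, clearing the Feet flag while falling.
; Most transition functions simply test Falling.
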(event Custom|Tick_Info
  (params (InOwner :type Pawn%20Object%20Reference))
  (Utilities|IsValid InOwner
    (:Is%20Valid
      (Utilities|IsValid (Variables|Default|GetCharacter)
        (:Is%20Valid
          _)
        (:Is%20Not%20Valid
          (Utilities|IsValid InOwner
            (:Is%20Valid
              (bind _asbp_character (Utilities|Casting|CastToBP_Character InOwner))
              (Variables|Default|SetCharacter _asbp_character)))))
      (Utilities|FlowControl|Sequence
        (:then_0
          (Variables|Default|SetSpeed (Math|Vector|VectorLengthXY (Transformation|GetVelocity (Variables|Default|GetCharacter))))
          (Variables|Default|SetPrevRotation "0, 0, 0")
          (Variables|Default|SetDirection (* (.Yaw (Math|Rotator|BreakRotator (Math|Interpolation|RInterpTo (Math|Rotator|Delta(Rotator) (Math|Rotator|MakeRotfromX (Transformation|GetVelocity (Variables|Default|GetCharacter))) (Transformation|GetActorRotation (Variables|Default|GetCharacter))) (Variables|Default|GetPrevRotation) (Utilities|Time|GetWorldDeltaSeconds) 25.0))) -1.0)))
        (:then_1
          (Variables|Default|SetControllerDirection (Math|Vector|DotProduct (Math|Vector|GetUpVector (Variables|/Script/Engine.Character|GetCapsuleComponent (Variables|Default|GetCharacter))) (Math|Vector|CrossProduct (Math|Vector|GetForwardVector (Pawn|GetControlRotation (Variables|Default|GetCharacter) :!class /Script/Engine.Pawn)) (Math|Vector|GetForwardVector (Variables|/Script/Engine.Character|GetCapsuleComponent (Variables|Default|GetCharacter))))))
          (Variables|Default|SetControllerDirection180 (* (Math|Vector|DotProduct (Math|Vector|GetUpVector (Variables|/Script/Engine.Character|GetCapsuleComponent (Variables|Default|GetCharacter))) (Math|Vector|CrossProduct (Math|Vector|GetForwardVector (Pawn|GetControlRotation (Variables|Default|GetCharacter) :!class /Script/Engine.Pawn)) (Math|Vector|GetForwardVector (Variables|/Script/Engine.Character|GetCapsuleComponent (Variables|Default|GetCharacter))))) 1.8e+02)))
        (:then_2
          (Utilities|IsValid (Actor|GetComponentbyClass (Variables|Default|GetCharacter) "/Game/Components/FeetComponent.FeetComponent_C")
            (:Is%20Valid
              (Variables|Default|SetFeetData (Variables|/Game/Components/FeetComponent.FeetComponent_C|GetData (Actor|GetComponentbyClass (Variables|Default|GetCharacter) "/Game/Components/FeetComponent.FeetComponent_C")))
              (Variables|Default|SetFeet true)
              (Variables|Default|SetLeftFoot (Variables|/Game/Components/FeetComponent.FeetComponent_C|GetLeftFoot (Actor|GetComponentbyClass (Variables|Default|GetCharacter) "/Game/Components/FeetComponent.FeetComponent_C")))
              (Variables|Default|SetRightFoot (Variables|/Game/Components/FeetComponent.FeetComponent_C|GetRightFoot (Actor|GetComponentbyClass (Variables|Default|GetCharacter) "/Game/Components/FeetComponent.FeetComponent_C")))
              (Variables|Default|SetLeftHand (Variables|/Game/Components/FeetComponent.FeetComponent_C|GetLeftHand (Actor|GetComponentbyClass (Variables|Default|GetCharacter) "/Game/Components/FeetComponent.FeetComponent_C")))
              (Variables|Default|SetRightHand (Variables|/Game/Components/FeetComponent.FeetComponent_C|GetRightHand (Actor|GetComponentbyClass (Variables|Default|GetCharacter) "/Game/Components/FeetComponent.FeetComponent_C")))
              (Variables|Default|SetPelvis (Variables|/Game/Components/FeetComponent.FeetComponent_C|GetPelvis (Actor|GetComponentbyClass (Variables|Default|GetCharacter) "/Game/Components/FeetComponent.FeetComponent_C")))
              (Variables|Default|SetGroundSlope (Variables|/Game/Components/FeetComponent.FeetComponent_C|GetGroundSlope (Actor|GetComponentbyClass (Variables|Default|GetCharacter) "/Game/Components/FeetComponent.FeetComponent_C"))))
            (:Is%20Not%20Valid
              (Variables|Default|SetFeet false))))
        (:then_3
          (bind _output_get (Variables|Default|SetFalling (AI|Components|NavMovement|IsFalling (Variables|/Script/Engine.Character|GetCharacterMovement (Variables|Default|GetCharacter)))))
          (if _output_get
            (Variables|Default|SetFeet false)))))
    (:Is%20Not%20Valid
      (Actor|DestroyActor self)
      (Development|PrintString "Destroy AnimaAnimInfo"))))

(fn ConstructionScript)

(fn FromMovetoJumpStart
  (return (Variables|Default|GetFalling)))

(fn FromFallingtoMove
  (return (not (Variables|Default|GetFalling))))

(fn FromMovetoFalling
  (return (Variables|Default|GetFalling)))

(fn FromMovetoRotate
  (return true))

(fn FromRotatetoJumpStart
  (return (Variables|Default|GetFalling)))