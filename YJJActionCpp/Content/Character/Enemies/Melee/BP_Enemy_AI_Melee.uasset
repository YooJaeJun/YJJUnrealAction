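; Melee enemy AI character Blueprint that extends its parent's hit, rise and death reactions.
; Getting hit enables combo on the main weapon if it is a random-pattern weapon.
; Ending a hit or rise shares one path that sets the blackboard Behavior enum after a validity check and shows it on state text.
; Death end cleans up weapons and destroys the actor.
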(event EventEndDead
  (bind _weaponcomponent (Variables|Default|GetWeaponComponent))
  (bind _weaponcomponent_2 (Variables|Default|GetWeaponComponent))
  (bind _mainweapon (Variables|/Game/Components/WeaponComponent.WeaponComponent_C|GetMainWeapon _weaponcomponent_2))
  (bind _subweapon (Variables|/Game/Components/WeaponComponent.WeaponComponent_C|GetSubWeapon _weaponcomponent))
  (|CallParentFunction)
  (Utilities|IsValid _mainweapon
    (:Is%20Valid
      (Default|Destroy _mainweapon)
      (Utilities|IsValid _subweapon
        (:Is%20Valid
          (Default|Destroy _subweapon))
        (:Is%20Not%20Valid
          _)))
    (:Is%20Not%20Valid
      _))
  (Actor|DestroyActor))

(event EventHitted
  (|CallParentFunction)
  (CallFunction|SetEnableRandomWeaponAction))

(event EventEndHitted
  (bind _returnvalue (Utilities|Enum|LiteralenumEBehaviorType "NewEnumerator11"))
  (bind _self self)
  (bind _self_2 self)
  (bind _returnvalue_2 (AI|GetAIController _self))
  (bind _returnvalue_3 (AI|GetAIController _self_2))
  (bind _returnvalue_4 (AI|GetBlackboard _returnvalue_2))
  (bind _returnvalue_5 (AI|GetBlackboard _returnvalue_3))
  (|CallParentFunction)
  (Utilities|IsValid (AI|GetBlackboard 0)
    (:Is%20Valid
      (Utilities|IsValid _returnvalue_4
        (:Is%20Valid
          (AI|Components|Blackboard|SetValueasEnum _returnvalue_4 (Utilities|Name|MakeLiteralName "Behavior") _returnvalue))))
    (:Is%20Not%20Valid
      (Utilities|IsValid _returnvalue_5
        (:Is%20Valid
          (AI|Components|Blackboard|SetValueasEnum _returnvalue_5 (Utilities|Name|MakeLiteralName "Behavior") (Utilities|Enum|LiteralenumEBehaviorType "NewEnumerator18"))))))
  (CallFunction|SetStateText (Variables|Default|GetStateTextRender) (Utilities|Text|ToText(String) _returnvalue)))

(event EventEndRise
  (bind _returnvalue (Utilities|Enum|LiteralenumEBehaviorType "NewEnumerator11"))
  (bind _self self)
  (bind _self_2 self)
  (bind _returnvalue_2 (AI|GetAIController _self))
  (bind _returnvalue_3 (AI|GetAIController _self_2))
  (bind _returnvalue_4 (AI|GetBlackboard _returnvalue_2))
  (bind _returnvalue_5 (AI|GetBlackboard _returnvalue_3))
  (|CallParentFunction)
  (Utilities|IsValid (AI|GetBlackboard 0)
    (:Is%20Valid
      (Utilities|IsValid _returnvalue_4
        (:Is%20Valid
          (AI|Components|Blackboard|SetValueasEnum _returnvalue_4 (Utilities|Name|MakeLiteralName "Behavior") _returnvalue))))
    (:Is%20Not%20Valid
      (Utilities|IsValid _returnvalue_5
        (:Is%20Valid
          (AI|Components|Blackboard|SetValueasEnum _returnvalue_5 (Utilities|Name|MakeLiteralName "Behavior") (Utilities|Enum|LiteralenumEBehaviorType "NewEnumerator18"))))))
  (CallFunction|SetStateText (Variables|Default|GetStateTextRender) (Utilities|Text|ToText(String) _returnvalue)))

(fn ConstructionScript
  (|CallParentFunction))

(fn SetEnableRandomWeaponAction
  (bind _asweapon_random_pattern (Utilities|Casting|CastToWeapon_RandomPattern (Variables|/Game/Components/WeaponComponent.WeaponComponent_C|GetMainWeapon (Variables|Default|GetWeaponComponent))))
  (Default|EnableCombo _asweapon_random_pattern)
  (return))