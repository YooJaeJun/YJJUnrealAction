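; Enemy character Blueprint that links combat hit reactions to its AI Blackboard.
; On BeginPlay it binds to the StateComponent's state-type change event.
; Entering Hitted, Hit Air, Down Flying or Down Land sets the Blackboard Behavior enum to one shared value and shows it on the StateTextRender.
; A valid Attacker also becomes the Blackboard Target, so the AI's target follows whoever hit it.
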(event Custom|OnStateTypeChanged_AI
  (params (InPrevType :type EStateType%20Enum :default "NewEnumerator20") (InNewType :type EStateType%20Enum :default "NewEnumerator20"))
  (bind _returnvalue (Utilities|Enum|LiteralenumEBehaviorType "NewEnumerator19"))
  (bind _self self)
  (bind _attacker (Variables|Default|GetAttacker))
  (bind _returnvalue_2 (AI|GetAIController _self))
  (bind _returnvalue_3 (AI|GetBlackboard _returnvalue_2))
  (switch Utilities|FlowControl|Switch|SwitchonEStateType InNewType
    (:NewEnumerator5
      _)
    (:NewEnumerator14
      _)
    (:NewEnumerator17
      _)
    (:NewEnumerator11
      _))
  (Utilities|IsValid _returnvalue_3
    (:Is%20Valid
      (AI|Components|Blackboard|SetValueasEnum _returnvalue_3 (Utilities|Name|MakeLiteralName "Behavior") _returnvalue)
      (CallFunction|SetStateText (Variables|Default|GetStateTextRender) (Utilities|Text|ToText(String) _returnvalue))
      (Utilities|IsValid _attacker
        (:Is%20Valid
          (AI|Components|Blackboard|SetValueasObject (AI|GetBlackboard 0) (Utilities|Name|MakeLiteralName "Target") _attacker))))))

(event EventBeginPlay
  (|CallParentFunction)
  (EventDispatchers|BindEventtoOnStateTypeChanged (Variables|Default|GetStateComponent) (delegate Custom|OnStateTypeChanged_AI)))

(fn ConstructionScript
  (|CallParentFunction))