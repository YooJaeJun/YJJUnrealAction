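; BP_Enemy_AI_Magic is an AI-controlled magic enemy that extends the behavior of a parent enemy Blueprint.
; After the parent handles the end of a hit or a rise, it sets the Behavior key on the AI controller's Blackboard to a fixed behavior type.
; When death ends, it destroys any active magic held by its MagicComponent, then destroys itself.
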(event EventEndDead
  (bind _magiccomponent (Variables|Default|GetMagicComponent))
  (bind _magic (Variables|/Game/Components/MagicComponent.MagicComponent_C|GetMagic _magiccomponent))
  (|CallParentFunction)
  (Utilities|IsValid _magic
    (:Is%20Valid
      (Default|Destroy _magic))
    (:Is%20Not%20Valid
      _))
  (Actor|DestroyActor))

(event EventEndHitted
  (bind _self self)
  (bind _returnvalue (AI|GetAIController _self))
  (bind _returnvalue_2 (AI|GetBlackboard _returnvalue))
  (|CallParentFunction)
  (Utilities|IsValid (AI|GetBlackboard 0)
    (:Is%20Not%20Valid
      (Utilities|IsValid _returnvalue_2
        (:Is%20Valid
          (AI|Components|Blackboard|SetValueasEnum _returnvalue_2 (Utilities|Name|MakeLiteralName "Behavior") (Utilities|Enum|LiteralenumEBehaviorType "NewEnumerator14")))))))

(event EventEndRise
  (bind _self self)
  (bind _returnvalue (AI|GetAIController _self))
  (bind _returnvalue_2 (AI|GetBlackboard _returnvalue))
  (|CallParentFunction)
  (Utilities|IsValid (AI|GetBlackboard 0)
    (:Is%20Not%20Valid
      (Utilities|IsValid _returnvalue_2
        (:Is%20Valid
          (AI|Components|Blackboard|SetValueasEnum _returnvalue_2 (Utilities|Name|MakeLiteralName "Behavior") (Utilities|Enum|LiteralenumEBehaviorType "NewEnumerator14")))))))

(fn ConstructionScript
  (|CallParentFunction))