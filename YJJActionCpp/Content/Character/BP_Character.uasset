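; BP_Character is a base character with shared hit reaction, riding interaction, possession and debug state-text logic, plus overridable hooks for menus and AI.
; SetDamagedInfo ignores same-group attackers, launches using the stored HitData before updating it, then sets Hitted on living characters.
; RestoreState maps StateComponent's previous state to Idle, Falling or Riding.
; Interact passes the character to the registered actor's RidingComponent.
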(fn ConstructionScript)

(fn RestoreState
  (bind _returnvalue (Actor|GetComponentbyClass "/Game/Components/StateComponent.StateComponent_C"))
  (switch Utilities|FlowControl|Switch|SwitchonEStateType (Variables|/Game/Components/StateComponent.StateComponent_C|GetPrevType _returnvalue)
    (:NewEnumerator0
      (Default|SetIdle _returnvalue :!label _label))
    (:NewEnumerator2
      (Default|SetFalling _returnvalue :!label _label_2))
    (:NewEnumerator3
      (Utilities|IsValid (Variables|Interact|GetCurRiddenActor) :!label _label_3
        (:Is%20Valid
          (Default|SetRiding _returnvalue))
        (:Is%20Not%20Valid
          (Default|SetIdle _returnvalue))))
    (:NewEnumerator5
      (goto _label_3))
    (:NewEnumerator6
      (goto _label_2))
    (:NewEnumerator10
      (goto _label_2))
    (:NewEnumerator13
      (goto _label_2))
    (:NewEnumerator14
      (goto _label_2))
    (:NewEnumerator17
      (goto _label_2))
    (:NewEnumerator11
      (goto _label_2))
    (:NewEnumerator12
      (goto _label))
    (:NewEnumerator19
      (Default|SetRiding _returnvalue))))

(fn RenderStateText
  (bind _statetextrender (Variables|Default|GetStateTextRender))
  (if (not (Variables|/Script/Engine.SceneComponent|GetbVisible _statetextrender))
    (Rendering|SetVisibility _statetextrender true false)))

(fn DontRenderStateText
  (bind _statetextrender (Variables|Default|GetStateTextRender))
  (if (Variables|/Script/Engine.SceneComponent|GetbVisible _statetextrender)
    (Rendering|SetVisibility _statetextrender false false)))

(fn BilboardStateText
  (bind _statetextrender (Variables|Default|GetStateTextRender))
  (Transformation|SetWorldRotation _statetextrender (Math|Rotator|MakeRotfromX (- (Transformation|GetActorLocation (Game|GetPlayerCameraManager 0)) (Transformation|GetWorldLocation _statetextrender))) false false))

(fn LaunchHit
  (Character|LaunchCharacter (* (Transformation|GetActorForwardVector) (* (.Launch (Utilities|Struct|BreakFHitData (Variables|Hit|GetHitData))) -1.0)) false false))

(fn SetRotation
  (Transformation|SetActorRotation (Math|Rotator|MakeRotator 0.0 0.0 (.yaw (Math|Rotator|FindLookatRotation (Transformation|GetActorLocation) (Transformation|GetActorLocation (Variables|Hit|GetAttacker)))))))

(fn PlayParticle
  (bind _hitdata (Variables|Hit|GetHitData))
  (bind (_damage _attacktype _montage _playrate _canmove _launch _cc _hitstop _sound _shakeclass _effect _effectlocation _effectscale) (Utilities|Struct|BreakFHitData _hitdata))
  (Effects|SpawnEmitteratLocation _effect (Variables|Hit|GetHitPoint) (Transformation|GetActorRotation) _effectscale))

(fn PlaySound
  (Audio|SpawnSoundatLocation (.Sound (Utilities|Struct|BreakFHitData (Variables|Hit|GetHitData))) (Variables|Hit|GetHitPoint) "0, 0, 0" 1.0 1.0 0.0 "/Game/Assets/Sounds/Weapons/SA_Sound.SA_Sound" 0))

(fn SetDamagedInfo
  (params (InAttacker :type BP%20Character%20Object%20Reference) (InCauser :type Actor%20Object%20Reference) (InHitData :type F%20Hit%20Data%20Structure) (InHitPoint :type Vector))
  (if (not (CallFunction|IsSameGroup InAttacker self))
    (Hit|LaunchHit)
    (if (not (Default|IsDead (Variables|Default|GetStateComponent)))
      (Variables|Hit|SetAttacker InAttacker)
      (Variables|Hit|SetCauser InCauser)
      (Variables|Hit|SetHitData InHitData)
      (Variables|Hit|SetHitPoint InHitPoint)
      (Default|SetHitted (Variables|Default|GetStateComponent)))))

(fn LaunchBack
  (bind _returnvalue (Transformation|GetActorForwardVector))
  (bind _constlaunchingback (Variables|Hit|GetConstLaunchingBack))
  (bind _returnvalue_2 (* _constlaunchingback -1.0))
  (bind _returnvalue_3 (* _returnvalue _returnvalue_2))
  (Character|LaunchCharacter (Math|Vector|MakeVector (.x _returnvalue_3) (.y _returnvalue_3) 1e+03) false false))

(event EventUnHoveredEquipMenu
  (params (InName :type String))
  ;[1 1 1] Override
)

(event EventClickedEquipMenu
  (params (InName :type String))
  ;[1 1 1] Override
)

(event EventHoveredMagicMenu
  (params (InName :type String))
  ;[1 1 1] Override
)

(event EventUnHoveredMagicMenu
  (params (InName :type String))
  ;[1 1 1] Override
)

(event EventClickedMagicMenu
  (params (InName :type String))
  ;[1 1 1] Override
)

(event EventHoveredEquipMenu
  (params (InName :type String))
  ;[1 1 1] Override
)

(event EventUpdateState
  (params (state :type EStateType%20Enum :default "NewEnumerator20"))
  (Default|SetMode (Variables|Default|GetStateComponent) state))

(event EventChangeAnimationBlueprint
  (params (InABPClass :type Object%20Class%20Reference))
  (Class|SkeletalMeshComponent|SetAnimClass (Variables|Character|GetMesh) InABPClass))

(event EventTogglePossess
  (params (InEnable :type Boolean))
  (bind _returnvalue (Game|GetPlayerController 0))
  (bind _self self)
  ;[1 1 1] Override
  (if InEnable
    (Pawn|Possess _returnvalue self)
    (Variables|BP_Character_C|SetCurController _self (Pawn|GetController _self))
    (else
      (Pawn|UnPossess _returnvalue))))

(event EventRegisterInteractableActor
  (params (InteractableActor :type Actor%20Object%20Reference))
  ;[1 1 1] Override
  (Variables|Interact|SetInteractableActor InteractableActor))

(event Input|ActionEvents|InputActionInteract
  (params (Key :type Key%20Structure :default "None"))
  (:Pressed
    (Utilities|IsValid (Variables|Interact|GetInteractableActor)
      (:Is%20Valid
        (Utilities|IsValid (Actor|GetComponentbyClass (Variables|Interact|GetInteractableActor) "/Game/Components/RidingComponent.RidingComponent_C")
          (:Is%20Valid
            (Class|IInteractable|StartInteraction(Message) (Actor|GetComponentbyClass (Variables|Interact|GetInteractableActor) "/Game/Components/RidingComponent.RidingComponent_C") self)
            (Variables|Interact|SetInteractableActor 0)))))))

(event Custom|End_Hitted
  ;[1 1 1] Override : AI
  (if (Default|IsHitted (Variables|Default|GetStateComponent))
    (세팅|RestoreState)))

(event EventBeginPlay
  (Utilities|FlowControl|Sequence
    (:then_0
      (Variables|/Script/Engine.CharacterMovementComponent|SetMaxWalkSpeed (Variables|Character|GetCharacterMovement) (Default|GetSprintSpeed (Variables|Default|GetMovingComponent))))))

(fn IsPlayer
  (return (Pawn|IsPlayerControlled)))