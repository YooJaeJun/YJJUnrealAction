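; Minimap actor that follows the player from 1000 units above and drives the player marker on the HUD minimap.
; BeginPlay finds the tagged player and adds a WB_Player_Icon to the WBMinimap canvas.
; Each Tick moves the actor over the player and pins the icon at a fixed point, rotated by player yaw.
; Enemy icon spawning and positioning graphs exist but are disconnected, so they never run.
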(event EventBeginPlay
  (Utilities|FlowControl|Sequence
    (:then_0
      (bind _outactors (Actor|GetAllActorswithTag "Player"))
      (bind _asbp_player (Utilities|Casting|CastToBP_Player (Utilities|Array|Get(acopy) _outactors)))
      (Variables|Default|SetPlayer _asbp_player)
      (bind _returnvalue (UserInterface|CreateWidget "/Game/Widgets/Player/WB_Player_Icon.WB_Player_Icon_C"))
      (bind _output_get (Variables|Default|SetPlayerIcon _returnvalue))
      (bind _asbp_game_mode (Utilities|Casting|CastToBP_GameMode (Game|GetGameMode)))
      (Class|CanvasPanel|AddChildtoCanvas (Variables|/Game/Widgets/Minimap/WB_Minimap.WB_Minimap_C|GetCanvasPanel_0 (Variables|/Game/Widgets/WB_HUDUI.WB_HUDUI_C|GetWB_Minimap (Default|GetHUD _asbp_game_mode))) _output_get))
    (:then_1)))

(event EventTick
  (params (DeltaSeconds :type Float%20%28single-precision%29))
  (bind _player (Variables|Default|GetPlayer))
  (bind _returnvalue (Transformation|GetActorLocation _player))
  (Utilities|IsValid _player
    (:Is%20Valid
      (Transformation|SetActorLocation (Math|Vector|MakeVector (.x _returnvalue) (.y _returnvalue) (+ (.z _returnvalue) 1e+03)) false false)
      (Utilities|FlowControl|Sequence
        (:then_0
          (Class|Widget|SetRenderTransform (Variables|Default|GetPlayerIcon) (Utilities|Struct|MakeWidgetTransform (Math|Vector2D|MakeVector2D 88.0 128.0) "(X=1.000000,Y=1.000000)" "(X=0.000000,Y=0.000000)" (- (.yaw (Transformation|GetActorRotation (Variables|Default|GetPlayer))) 9e+01))))
        (:then_1)))))

(fn ConstructionScript)