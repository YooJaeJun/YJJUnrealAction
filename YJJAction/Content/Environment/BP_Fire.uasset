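; BP_Fire is a fire actor that spreads across grass by spawning copies of itself.
; Shortly after BeginPlay, Propagate increments a counter that selects one of four horizontal offsets, then line-traces downward there.
; A Grass physical surface hit spawns another BP_Fire at that offset, which runs the same logic.
; A delayed repeat of Propagate runs only while the counter is below zero, checked after the increment.
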(event Custom|Propagate
  (bind _returnvalue (Transformation|GetActorLocation))
  (bind _propagatedcount (Variables|Default|GetPropagatedCount))
  (bind _returnvalue_2 (Utilities|Select :Index _propagatedcount :Option%200 "1.000000,0.000000, 0" :Option%201 "1.000000,1.000000,0.000000" :Option%202 "-1.000000,0.000000, 0" :Option%203 "-1.000000,-1.000000,0.000000"))
  (bind _returnvalue_3 (* _returnvalue_2 1e+02))
  (bind _returnvalue_4 (+ _returnvalue_3 _returnvalue))
  (Math|Integer|IncrementInt _propagatedcount
    (:%20%20
      (Utilities|FlowControl|Sequence
        (:then_0
          (bind (_outhit _returnvalue_5) (Collision|LineTraceByChannel (+ _returnvalue_4 "0, 0,100.000000") (+ _returnvalue_4 "0, 0,-100.000000") "TraceTypeQuery1" false 0 "None"))
          (if _returnvalue_5
            (switch Utilities|FlowControl|Switch|SwitchonEPhysicalSurface (Variables|/Script/PhysicsCore.PhysicalMaterial|GetSurfaceType (.PhysMat (Collision|BreakHitResult _outhit)))
              (:SurfaceType1
                (Game|SpawnActorfromClass "BP_Fire_C" (Math|Transform|MakeTransform _returnvalue_4 "0, 0, 0" "1,1,1") "Undefined" 0 0)))))
        (:then_1
          (Utilities|FlowControl|Delay 2.0)
          (if (< (Variables|Default|GetPropagatedCount) 0)
            (CallFunction|Propagate)))))))

(event EventBeginPlay
  (Utilities|FlowControl|Delay 3.0)
  (CallFunction|Propagate))

(fn ConstructionScript)