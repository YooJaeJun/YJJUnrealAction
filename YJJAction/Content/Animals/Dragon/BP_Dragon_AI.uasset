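; Dragon boss character (Ragnarök) that announces itself, drives the HUD boss HP and groggy bars, and can be ridden and flown.
; Rider combat, targeting and menu inputs forward to RidingComponent, while roar and fire go to a spawned DragonWeapon.
; Flight toggles state and gravity, banks and pitches by input, and lands via a downward trace.
; Hits build groggy toward a stagger montage; landings play surface sounds, effects and camera shake.
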(fn ConstructionScript)

(fn IsFlying
  (bind _statecomponent (Variables|Default|GetStateComponent))
  (return (or (Default|IsFalling _statecomponent) (Default|IsFlying _statecomponent))))

(fn UpdateHp
  (Default|SetHPUI (Variables|UI|GetHpBar) (Variables|Default|GetHp) (Variables|Default|GetMaxHp)))

(fn UpdateGroggy
  (Default|SetGroggyUI (Variables|UI|GetGroggyBar) (Variables|Groggy|GetGroggy) (Variables|Groggy|GetMaxGroggy)))

(fn SpawnMessage
  (Default|Play (Variables|Default|GetSystemMessageComponent) "Ragnarök가 강림했습니다." 5.0))

(fn SetGroggy
  (Variables|Groggy|SetGroggy 0.0))

(fn EndGroggy
  (Default|SetIdle (Variables|Default|GetStateComponent)))

(fn SetGroggyDamage
  (Variables|Groggy|SetGroggy (Math|Float|Clamp(Float) (+ (Variables|Groggy|GetGroggy) (/ (.Damage (Utilities|Struct|BreakFHitData (Variables|Default|GetHitData))) 5.0)) 0.0 (Variables|Groggy|GetMaxGroggy)))
  (if (>= (Variables|Groggy|GetGroggy) (Variables|Groggy|GetMaxGroggy))
    (Variables|Groggy|SetGroggy 0.0)
    (Variables|Groggy|SetInGroggy true)
    (Utilities|Time|SetTimerbyFunctionName 0 "End_Groogy" (Variables|Groggy|GetGroggyTime))
    (Default|SetGroggy (Variables|Default|GetStateComponent))
    (Animation|StopAnimMontage 0)
    (Animation|PlayAnimMontage (Variables|Groggy|GetGroggyAnim) 1.0 "None")))

(event Input|ActionEvents|InputActionInteract
  (params (Key :type Key%20Structure :default "None"))
  (:Pressed
    (Class|IInteractable|EndInteraction(Message) (Variables|Default|GetRidingComponent))))

(event OnComponentBeginOverlap(InterationCollision)
  (params (OverlappedComponent :type Primitive%20Component%20Object%20Reference) (OtherActor :type Actor%20Object%20Reference) (OtherComp :type Primitive%20Component%20Object%20Reference) (OtherBodyIndex :type Integer) (bFromSweep :type Boolean) (SweepResult :type Hit%20Result%20Structure%20%28by%20ref%29))
  (Default|BeginOverlap (Variables|Default|GetRidingComponent) OtherActor))

(event OnComponentEndOverlap(InterationCollision)
  (params (OverlappedComponent :type Primitive%20Component%20Object%20Reference) (OtherActor :type Actor%20Object%20Reference) (OtherComp :type Primitive%20Component%20Object%20Reference) (OtherBodyIndex :type Integer))
  (Default|EndOverlap (Variables|Default|GetRidingComponent) OtherActor))

(event Input|ActionEvents|InputActionAction
  (params (Key :type Key%20Structure :default "None"))
  ;[1 1 1] Action
  (:Pressed
    (Default|Action (Variables|Default|GetRidingComponent))))

(event Input|ActionEvents|InputActionSkill_1
  (params (Key :type Key%20Structure :default "None"))
  ;[1 1 1] Skill
  (:Pressed
    (Default|Skill (Variables|Default|GetRidingComponent))))

(event Input|ActionEvents|InputActionSkill_2
  (params (Key :type Key%20Structure :default "None"))
  ;[1 1 1] Skill
  (:Pressed
    (Default|Skill (Variables|Default|GetRidingComponent) 1)))

(event Input|ActionEvents|InputActionSubWeapon_Action
  (params (Key :type Key%20Structure :default "None"))
  ;[1 1 1] SubWeapon - Action
  (:Pressed
    (Default|SubWeaponActionPressed (Variables|Default|GetRidingComponent)))
  (:Released
    (Default|SubWeaponActionReleased (Variables|Default|GetRidingComponent))))

(event Input|ActionEvents|InputActionMagic
  (params (Key :type Key%20Structure :default "None"))
  ;[1 1 1] Magic
  (:Pressed
    (Default|Magic (Variables|Default|GetRidingComponent))))

(event EventOnLanded
  (params (Hit :type Hit%20Result%20Structure%20%28by%20ref%29))
  (switch Utilities|FlowControl|Switch|SwitchonEStateType (Variables|/Game/Components/StateComponent.StateComponent_C|GetType (Variables|Default|GetStateComponent))
    (:NewEnumerator20
      (Default|SetCinematic (Variables|Default|GetStateComponent)))
    (:NewEnumerator13
      (Default|SetIdle (Variables|Default|GetStateComponent))))
  (Default|SetGravity (Variables|Default|GetMovingComponent) 1.0)
  (CallFunction|Land "SurfaceType_Default" (Transformation|GetActorLocation)))

(event EventLand
  (params (SurfaceType :type EPhysicalSurface%20Enum :default "SurfaceType_Default") (StepLocation :type Vector :default "0, 0, 0"))
  (|CallParentFunction SurfaceType StepLocation)
  (switch Utilities|FlowControl|Switch|SwitchonEPhysicalSurface SurfaceType
    (:SurfaceType_Default
      (Audio|PlaySoundatLocation "/Game/Assets/Sounds/Animals/Ultimate_SFX/Dragon_Sounds_Pro/Cues/DRAGON_FOOTSTEPS/Rock.Rock" "0, 0, 0" "0, 0, 0" 1.0 1.0 0.0 0 0 0))
    (:SurfaceType1
      (Audio|PlaySoundatLocation "/Game/Assets/Sounds/Animals/Ultimate_SFX/Dragon_Sounds_Pro/Cues/DRAGON_FOOTSTEPS/Grass.Grass" StepLocation "0, 0, 0" 1.0 1.0 0.0 0 0 0))
    (:SurfaceType2
      (Audio|PlaySoundatLocation "/Game/Assets/Sounds/Animals/Ultimate_SFX/Dragon_Sounds_Pro/Cues/DRAGON_FOOTSTEPS/Wood.Wood" StepLocation "0, 0, 0" 1.0 1.0 0.0 0 0 0))
    (:SurfaceType3
      (Audio|PlaySoundatLocation "/Game/Assets/Sounds/Animals/Ultimate_SFX/Dragon_Sounds_Pro/Cues/DRAGON_FOOTSTEPS/Sand.Sand" StepLocation "0, 0, 0" 1.0 1.0 0.0 0 0 0))
    (:SurfaceType4
      (Audio|PlaySoundatLocation "/Game/Assets/Sounds/Animals/Ultimate_SFX/Dragon_Sounds_Pro/Cues/DRAGON_FOOTSTEPS/Rock.Rock" StepLocation "0, 0, 0" 1.0 1.0 0.0 0 0 0))
    (:SurfaceType5
      (Audio|PlaySoundatLocation "/Game/Assets/Sounds/Animals/Ultimate_SFX/Dragon_Sounds_Pro/Cues/DRAGON_FOOTSTEPS/Water.Water" StepLocation "0, 0, 0" 1.0 1.0 0.0 0 0 0)))
  (Niagara|SpawnSystematLocation (Variables|Default|GetFootstepEffect) StepLocation)
  (CameraShakes|StartCameraShake (Game|GetPlayerCameraManager 0) "/Game/Player/CS_NotEnoughState.CS_NotEnoughState_C" 1.0 "CameraLocal" "0, 0, 0"))

(event Input|ActionEvents|InputActionTargeting
  (params (Key :type Key%20Structure))
  (:Pressed
    (Default|TargetingInput (Variables|Default|GetRidingComponent))))

(event Input|AxisEvents|InputAxisZoom
  (params (AxisValue :type Float%20%28single-precision%29))
  (Default|ZoomInput (Variables|Default|GetRidingComponent) AxisValue))

(event EventBeginPlay
  (|CallParentFunction)
  (Utilities|FlowControl|Sequence
    (:then_0
      (bind _returnvalue (Game|SpawnActorfromClass (Variables|Weapons|GetDragonWeaponClass) (Transformation|GetActorTransform) "Undefined" self 0))
      (Variables|Weapons|SetDragonWeapon _returnvalue))
    (:then_1
      (Transformation|AttachComponentToComponent (Variables|Default|GetNeck) (Variables|Character|GetMesh) "Fire_Ground" "SnapToTarget" "SnapToTarget" "KeepRelative" true))
    (:then_2
      (bind _asbp_game_mode (Utilities|Casting|CastToBP_GameMode (Game|GetGameMode)))
      (Variables|UI|SetHpBar (Variables|/Game/Widgets/Boss/WB_Boss_Info.WB_Boss_Info_C|GetWB_Boss_HpBar (Variables|/Game/Widgets/WB_HUDUI.WB_HUDUI_C|GetWB_BossInfo (Default|GetHUD _asbp_game_mode))))
      (Variables|UI|SetGroggyBar (Variables|/Game/Widgets/Boss/WB_Boss_Info.WB_Boss_Info_C|GetWB_Boss_GroggyBar (Variables|/Game/Widgets/WB_HUDUI.WB_HUDUI_C|GetWB_BossInfo (Default|GetHUD _asbp_game_mode))))
      (Widget|SetVisibility (Variables|/Game/Widgets/WB_HUDUI.WB_HUDUI_C|GetWB_BossInfo (Default|GetHUD _asbp_game_mode)) "Visible")
      (Default|SetName (Variables|/Game/Widgets/WB_HUDUI.WB_HUDUI_C|GetWB_BossInfo (Default|GetHUD _asbp_game_mode)) (Utilities|Text|ToText(String) (.Name (Utilities|Struct|BreakFCharacterInfo (Variables|Default|GetCharacterInfo)))))
      (UI|UpdateHp)
      (UI|UpdateGroggy))
    (:then_3
      (UI|SpawnMessage))))

(event Custom|FlyJump
  (params (InNewState :type EStateType%20Enum :default "NewEnumerator0") (InGravity :type Float%20%28single-precision%29))
  (bind _statecomponent (Variables|Default|GetStateComponent))
  ;[1 1 1] Fly Jump
  (if (not (Fly|IsFlying))
    (if (Default|IsCanMove (Variables|Default|GetMovingComponent))
      (Utilities|FlowControl|Sequence
        (:then_0
          (Character|Jump)
          (switch Utilities|FlowControl|Switch|SwitchonEStateType InNewState
            (:NewEnumerator10
              (Default|SetFlying _statecomponent))
            (:NewEnumerator13
              (Default|SetFalling _statecomponent))))
        (:then_1
          (Default|SetGravity (Variables|Default|GetMovingComponent) InGravity)
          (Niagara|SpawnSystematLocation (Variables|Fly|GetJumpEffect) (Transformation|GetWorldLocation (Variables|Character|GetMesh))))))
    (else
      (CallFunction|Landon))))

(event Custom|LandOn
  (bind _returnvalue (Transformation|GetActorLocation))
  ;[1 1 1] 착지
  (bind (_outhit _returnvalue_2) (Collision|LineTraceByChannel (Transformation|GetActorLocation) (Math|Vector|MakeVector (.x _returnvalue) (.y _returnvalue) (.z (+ (* (Math|Vector|GetUpVector (Variables|Character|GetMesh)) -6e+03) (.z _returnvalue)))) "TraceTypeQuery1" false 0 "ForOneFrame"))
  (if _returnvalue_2
    (Default|SetFalling (Variables|Default|GetStateComponent))
    (Default|SetGravity (Variables|Default|GetMovingComponent) 1.0)
    (Components|MoveComponentTo (Variables|Transformation|GetRootComponent) (+ (.ImpactPoint (Collision|BreakHitResult _outhit)) (Components|Capsule|GetScaledCapsuleHalfHeight (Variables|Default|GetCapsuleComponent))) (Transformation|GetActorRotation) true true 1.0 false)))

(event Input|ActionEvents|InputActionJumping
  (params (Key :type Key%20Structure))
  ;[1 1 1] Fly Jump
  (:Pressed
    (CallFunction|FlyJump "NewEnumerator10" 0.0)))

(event Input|AxisEvents|InputAxisMoveForward
  (params (AxisValue :type Float%20%28single-precision%29))
  ;[1 1 1] Moving
  (if (CallFunction|CanMove AxisValue)
    (Pawn|Input|AddMovementInput (.OutForward (CallFunction|GetControlDirection)) AxisValue true)
    (if (Fly|IsFlying)
      (Transformation|SetActorLocation (+ (Transformation|GetActorLocation) (* (Math|Vector|GetForwardVector (Variables|Default|GetCapsuleComponent)) (* AxisValue 4e+01))) false false))))

(event Input|AxisEvents|InputAxisMoveRight
  (params (AxisValue :type Float%20%28single-precision%29))
  (bind _returnvalue (Transformation|GetActorRotation))
  (bind _returnvalue_2 (Transformation|GetActorRotation))
  ;[1 1 1] Moving
  (if (CallFunction|CanMove AxisValue)
    (Pawn|Input|AddMovementInput (.OutRight (CallFunction|GetControlDirection)) AxisValue true)
    (if (Fly|IsFlying)
      (Transformation|SetActorTransform (Math|Transform|MakeTransform (+ (Transformation|GetActorLocation) (* (Math|Vector|GetForwardVector (Variables|Default|GetCapsuleComponent)) (* (Math|Float|Absolute(Float) AxisValue) 4e+01))) (Math|Rotator|MakeRotator (Math|Float|Clamp(Float) (+ (.roll _returnvalue) AxisValue) -6e+01 6e+01) (.pitch _returnvalue) (.yaw _returnvalue)) "1,1,1")))
    (elif (Fly|IsFlying)
      (Transformation|SetActorRotation (Math|Interpolation|RInterpTo (Transformation|GetActorRotation) (Math|Rotator|MakeRotator 0.0 (.pitch _returnvalue_2) (.yaw _returnvalue_2)) (Utilities|Time|GetWorldDeltaSeconds) 2.0)))))

(event Input|AxisEvents|InputAxisFlyUp
  (params (AxisValue :type Float%20%28single-precision%29))
  (bind _returnvalue (Transformation|GetActorRotation))
  (bind _returnvalue_2 (Transformation|GetActorRotation))
  ;[1 1 1] FlyUpDown
  (if (CallFunction|CanMove AxisValue)
    (if (> AxisValue 0.0)
      (Variables|Fly|SetUpFactor 2e+01)
      (else
        (Variables|Fly|SetUpFactor -5e+01)))
    (Transformation|SetActorTransform (Math|Transform|MakeTransform (+ (Transformation|GetActorLocation) (* (Math|Vector|GetForwardVector (Variables|Default|GetCapsuleComponent)) (* AxisValue (Variables|Fly|GetUpFactor)))) (Math|Rotator|MakeRotator (.roll _returnvalue) (Math|Float|Clamp(Float) (+ (.pitch _returnvalue) AxisValue) -6e+01 6e+01) (.yaw _returnvalue)) "1,1,1"))
    (elif (Fly|IsFlying)
      (Transformation|SetActorRotation (Math|Interpolation|RInterpTo (Transformation|GetActorRotation) (Math|Rotator|MakeRotator (.roll _returnvalue_2) 0.0 (.yaw _returnvalue_2)) (Utilities|Time|GetWorldDeltaSeconds) 2.0)))))

(event Input|ActionEvents|InputActionDragonFire
  (params (Key :type Key%20Structure))
  (:Pressed
    (Default|Skill (Variables|Weapons|GetDragonWeapon) "NewEnumerator1")))

(event Input|ActionEvents|InputActionDragonRoar
  (params (Key :type Key%20Structure))
  (:Pressed
    (Default|Skill (Variables|Weapons|GetDragonWeapon) "NewEnumerator0")))

(event EventSetupCinematic
  (params (OnOff :type Boolean))
  (if OnOff
    (Default|SetCinematic (Variables|Default|GetStateComponent))
    (Default|SetGravity (Variables|Default|GetMovingComponent) 0.0)
    (Utilities|FlowControl|Delay 11.0)
    (Default|SetGravity (Variables|Default|GetMovingComponent) 0.4)
    (else
      (Default|SetIdle (Variables|Default|GetStateComponent)))))

(event Custom|MagicMenu_Hide
  ;[1 1 1] Wrapping
  (Default|MagicMenuHide (Variables|Default|GetRidingComponent)))

(event Custom|Menu_Hide
  ;[1 1 1] Wrapping
  (Default|MenuHide (Variables|Default|GetRidingComponent)))

(event EventUnHoveredEquipMenu
  (params (InName :type String))
  ;[1 1 1] UI
  (Default|UnhoveredEquip (Variables|Default|GetRidingComponent) InName))

(event EventClickedEquipMenu
  (params (InName :type String))
  ;[1 1 1] UI
  (Default|ClickedEquip (Variables|Default|GetRidingComponent) InName))

(event EventHoveredMagicMenu
  (params (InName :type String))
  ;[1 1 1] UI
  (Default|HoveredMagic (Variables|Default|GetRidingComponent) InName))

(event EventUnHoveredMagicMenu
  (params (InName :type String))
  ;[1 1 1] UI
  (Default|UnhoveredMagic (Variables|Default|GetRidingComponent) InName))

(event EventClickedMagicMenu
  (params (InName :type String))
  ;[1 1 1] UI
  (Default|ClickedMagic (Variables|Default|GetRidingComponent) InName))

(event EventHoveredEquipMenu
  (params (InName :type String))
  ;[1 1 1] UI
  (Default|HoveredEquip (Variables|Default|GetRidingComponent) InName))

(event Input|ActionEvents|InputActionMagicMenu
  (params (Key :type Key%20Structure))
  ;[1 1 1] Wrapping
  (:Pressed
    (Default|MagicMenu (Variables|Default|GetRidingComponent)))
  (:Released
    (Default|MagicMenuHide (Variables|Default|GetRidingComponent))))

(event Input|ActionEvents|InputActionMenu
  (params (Key :type Key%20Structure))
  ;[1 1 1] Wrapping
  (:Pressed
    (Default|Menu (Variables|Default|GetRidingComponent)))
  (:Released
    (Default|MenuHide (Variables|Default|GetRidingComponent))))

(event EventHitted
  (|CallParentFunction)
  (Utilities|FlowControl|Sequence
    (:then_0
      (Groggy|SetGroggyDamage))
    (:then_1
      (UI|UpdateHp)
      (UI|UpdateGroggy))))