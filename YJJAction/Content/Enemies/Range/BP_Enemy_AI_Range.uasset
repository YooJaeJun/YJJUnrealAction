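; Ranged enemy AI Blueprint that overrides its parent's hit, rise and death end events.
; When a hit reaction or rise ends, it calls the parent, then shares one path that writes a fixed Behavior enum value to the AI controller's blackboard, behind validity checks.
; When death ends, it calls the parent, destroys valid main and sub weapons from the weapon component, then destroys itself.
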(event EventEndDead
  (bind _weaponcomponent (Variables|Default|GetWeaponComponent))
  (bind _weaponcomponent_2 (Variables|Default|GetWeaponComponent))
  (bind _mainweapon (Variables|/Game/Components/WeaponComponent.WeaponComponent_C|GetMainWeapon _weaponcomponent))
  (bind _subweapon (Variables|/Game/Components/WeaponComponent.WeaponComponent_C|GetSubWeapon _weaponcomponent_2))
  (|CallParentFunction)
  (Utilities|IsValid _mainweapon
    (:Is%20Valid
      (Default|Destroy _mainweapon)
      (Utilities|IsValid _subweapon
        (:Is%20Valid
          (Default|Destroy _subweapon))
        (:Is%20Not%20Valid
          _)))
    (:Is%20Not%20Valid
      _))
  (Actor|DestroyActor))

(event EventEndHitted
  (bind _self self)
  (bind _returnvalue (AI|GetAIController _self))
  (bind _returnvalue_2 (AI|GetBlackboard _returnvalue))
  (|CallParentFunction)
  (Utilities|IsValid (AI|GetBlackboard 0)
    (:Is%20Not%20Valid
      (Utilities|IsValid _returnvalue_2
        (:Is%20Valid
          (AI|Components|Blackboard|SetValueasEnum _returnvalue_2 (Utilities|Name|MakeLiteralName "Behavior") (Utilities|Enum|LiteralenumEBehaviorType "NewEnumerator14")))))))

(event EventEndRise
  (bind _self self)
  (bind _returnvalue (AI|GetAIController _self))
  (bind _returnvalue_2 (AI|GetBlackboard _returnvalue))
  (|CallParentFunction)
  (Utilities|IsValid (AI|GetBlackboard 0)
    (:Is%20Not%20Valid
      (Utilities|IsValid _returnvalue_2
        (:Is%20Valid
          (AI|Components|Blackboard|SetValueasEnum _returnvalue_2 (Utilities|Name|MakeLiteralName "Behavior") (Utilities|Enum|LiteralenumEBehaviorType "NewEnumerator14")))))))

(fn ConstructionScript
  (|CallParentFunction))