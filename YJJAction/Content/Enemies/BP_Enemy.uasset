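; BP_Enemy is an enemy character with an HP bar that reacts to hits, drops items and rewards its killer on death.
; StateComponent changes dispatch hit, death, air-launch, knockdown and rise reactions.
; Hits apply HitData damage, montage, red material flash, effects and crowd control, with gravity changes for falls.
; Player attacks add camera shake and hit-stop, which near-freezes pawns and movable-mesh actors through CustomTimeDilation until a timer restores them.
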(fn ConstructionScript)

(fn PlayHitAnim
  (bind _hitdata (Variables|Default|GetHitData))
  (bind (_damage _attacktype _montage _playrate) (Utilities|Struct|BreakFHitData _hitdata))
  (Animation|PlayAnimMontage _montage _playrate "None")
  (return))

(fn SetColor
  (for _array_element (Variables|BasicInfo|GetMaterials)
    (Rendering|Material|SetVectorParameterValue _array_element "BodyColor" "(R=1.000000,G=0.000000,B=0.000000,A=1.000000)" :!class /Script/Engine.MaterialInstanceDynamic))
  (Utilities|Time|SetTimerbyFunctionName 0 "SetOriginColor" 0.15))

(fn SetOriginColor
  (for _array_element (Variables|BasicInfo|GetMaterials)
    (Rendering|Material|SetVectorParameterValue _array_element "BodyColor" (.BodyColor (Utilities|Struct|BreakFCharacterInfo (Variables|Default|GetCharacterInfo))) :!class /Script/Engine.MaterialInstanceDynamic))
  (return))

(fn PlayHitStop
  (bind _returnvalue (Actor|GetComponentbyClass "/Script/Engine.MeshComponent"))
  (Utilities|Casting|CastToBP_Player (Variables|Default|GetAttacker))
  (if (not (Math|Float|NearlyEqual(Float) (.HitStop (Utilities|Struct|BreakFHitData (Variables|Default|GetHitData))) 0.0 1e-06))
    (bind _outactors (Actor|GetAllActorsOfClass "/Script/Engine.Actor"))
    (for _array_element _outactors
      (Utilities|Casting|CastToPawn _array_element
        (:then
          (Utilities|Array|Add (Variables|Hit|GetDilationActors) _array_element :!label _label)
          (Variables|/Script/Engine.Actor|SetCustomTimeDilation _array_element 0.001))
        (:CastFailed
          (Utilities|IsValid _returnvalue
            (:Is%20Valid
              (if (Utilities|Enum|Equal(Enum) (Variables|/Script/Engine.SceneComponent|GetMobility _returnvalue) "Movable")
                (goto _label)))))))
    (Utilities|Time|SetTimerbyFunctionName self "RestoreTimeDilation" (.HitStop (Utilities|Struct|BreakFHitData (Variables|Default|GetHitData))))
    (return)))

(fn RestoreTimeDilation
  (bind _dilationactors (Variables|Hit|GetDilationActors))
  (for _array_element _dilationactors
    (Utilities|IsValid _array_element
      (:Is%20Valid
        (Variables|/Script/Engine.Actor|SetCustomTimeDilation _array_element 1.0))))
  (Utilities|Array|Clear _dilationactors))

(fn PlayCameraShake
  (bind _hitdata (Variables|Default|GetHitData))
  (bind _shakeclass (Utilities|Struct|BreakFHitData _hitdata))
  (Utilities|Casting|CastToBP_Player (Variables|Default|GetAttacker))
  (if (Utilities|IsValidClass _shakeclass)
    (CameraShakes|StartCameraShake (Game|GetPlayerCameraManager 0) _shakeclass 1.0 "CameraLocal" "0, 0, 0")))

(fn LoadPrevState
  (bind _statecomponent (Variables|Default|GetStateComponent))
  (if (not (Default|IsDead _statecomponent))
    (Default|SetIdle _statecomponent)))

(fn SetDamage
  (Variables|Status|SetHp (Math|Float|Clamp(Float) (- (Variables|Status|GetHp) (.Damage (Utilities|Struct|BreakFHitData (Variables|Default|GetHitData)))) 0.0 (Variables|Status|GetMaxHp)))
  (Default|SetHpPercent (Variables|Status|GetHpBar_UI) (/ (Variables|Status|GetHp) (Variables|Status|GetMaxHp)))
  (return (> (Variables|Status|GetHp) 0.0)))

(fn HitCC
  (switch Utilities|FlowControl|Switch|SwitchonEAttackType (.AttackType (Utilities|Struct|BreakFHitData (Variables|Default|GetHitData)))
    (:NewEnumerator1
      (Variables|CC|SetCoordBeforeAir (Transformation|GetActorLocation))
      (Default|SetHitAir (Variables|Default|GetStateComponent))
      (Variables|CC|SetFlyToFall false))
    (:NewEnumerator2
      (Default|SetDownFlying (Variables|Default|GetStateComponent) :!label _label)
      (if (Utilities|Enum|Equal(Enum) (.CC (Utilities|Struct|BreakFHitData (Variables|Default|GetHitData))) "NewEnumerator1")
        (CC|StartFall 5e+01)))
    (:NewEnumerator11
      (goto _label))))

(fn TickAirBone
  (bind _attacker (Variables|Default|GetAttacker))
  (if (Default|IsHitAir (Variables|Default|GetStateComponent))
    ;[1 1 1] 낙하 가능 체크. StartFall에서 Fly to Fall 켜주어 한 번만 실행
    (if (not (Variables|CC|GetFlyToFall))
      (if (Math|Float|NearlyEqual(Float) (.z (Transformation|GetActorLocation)) (+ (.z (Variables|CC|GetCoordBeforeAir)) (Variables|CC|GetAirDistance)) 5.0)
        (CC|StartFall 2.0)))
    (else
      ;[1 1 1] 히트 시 공격자 따라가기
      (if (Default|IsDownFlying (Variables|Default|GetStateComponent))
        (Transformation|SetActorLocation (+ (Transformation|GetActorLocation _attacker) (* (Transformation|GetActorForwardVector _attacker) 1e+02)) false false)))))

(fn StartFall
  (params (InGravity :type Float%20%28single-precision%29))
  (Pawn|Components|CharacterMovement|SetMovementMode (Variables|Character|GetCharacterMovement) "MOVE_Falling" 0)
  (Default|SetFalling (Variables|Default|GetStateComponent))
  (Default|SetGravity (Variables|Default|GetMovingComponent) InGravity)
  (Variables|CC|SetFlyToFall true))

(fn SetMaterial
  (for _array_element (Rendering|Material|GetMaterials (Variables|Character|GetMesh))
    (bind _returnvalue (Rendering|Material|CreateDynamicMaterialInstance _array_element "None" "None" :!class /Script/Engine.KismetMaterialLibrary))
    (bind _returnvalue_2 (Utilities|Array|Add (Variables|BasicInfo|GetMaterials) _returnvalue))
    (Rendering|Material|SetMaterial (Variables|Character|GetMesh) _returnvalue_2 _returnvalue)
    (Rendering|Material|SetVectorParameterValue _returnvalue "BodyColor" (.BodyColor (Utilities|Struct|BreakFCharacterInfo (Variables|Default|GetCharacterInfo))) :!class /Script/Engine.MaterialInstanceDynamic))
  (return))

(fn SetStatus
  (Variables|Status|SetHp (Variables|Status|GetMaxHp))
  (bind _aswb_hp_bar_guage_enemy (Utilities|Casting|CastToWB_HpBar_Guage_Enemy (UserInterface|GetUserWidgetObject (Variables|Default|GetHpBarWidget))))
  (bind _output_get (Variables|Status|SetHpBar_UI _aswb_hp_bar_guage_enemy))
  (Default|SetHpPercent _output_get (/ (Variables|Status|GetHp) (Variables|Status|GetMaxHp)))
  (return))

(fn SetTargetWidget
  (Rendering|SetVisibility (Variables|Default|GetTargetingWidget) false false)
  (return))

(fn UpdateWalkSpeed
  (params (NewWalkSpeed :type Float%20%28single-precision%29))
  (Variables|/Script/Engine.CharacterMovementComponent|SetMaxWalkSpeed (Variables|Character|GetCharacterMovement) NewWalkSpeed))

(fn SetMinimapIcon
  ;[1 1 1] 현재 안됨
)

(fn DropItem
  (Default|Drop (Variables|Default|GetDropItemComponent)))

(fn SpawnBlood
  (if (Variables|Status|GetBloody)
    (Game|SpawnActorfromClass "/Game/Effects/sA_BloodSplatter_System/Blueprints/BP_Splater_Preset_2.BP_Splater_Preset_2_C" (Transformation|GetActorTransform) "Undefined" 0 0)
    (Audio|PlaySoundatLocation "/Game/Sounds/Hits/Blood_Fart_6.Blood_Fart_6" (Transformation|GetActorLocation) "0, 0, 0" 1.0 1.0 0.0 0 0 0)))

(event Custom|Begin_Bound)

(event Custom|End_Rise
  (Default|SetIdle (Variables|Default|GetStateComponent)))

(event Custom|End_Bound
  (bind _statecomponent (Variables|Default|GetStateComponent))
  (if (not (Default|IsDead _statecomponent))
    (if (or (Default|IsDownFlying _statecomponent) (Default|IsHitAir _statecomponent))
      (if (Character|CanJump)
        (Default|SetRise (Variables|Default|GetStateComponent) :!label _label))
      (else
        (goto _label)))))

(event EventTick
  (params (DeltaSeconds :type Float%20%28single-precision%29))
  (CC|TickAirBone)
  (CallFunction|BilboardStateText))

(event EventOnLanded
  (params (Hit :type Hit%20Result%20Structure%20%28by%20ref%29))
  (Default|SetGravity (Variables|Default|GetMovingComponent) 1.0)
  (switch Utilities|FlowControl|Switch|SwitchonEStateType (Variables|/Game/Components/StateComponent.StateComponent_C|GetType (Variables|Default|GetStateComponent))
    (:NewEnumerator0
      _)
    (:NewEnumerator3
      _)
    (:NewEnumerator4
      _)
    (:NewEnumerator5
      _)
    (:NewEnumerator10
      _)
    (:NewEnumerator13
      _)
    (:NewEnumerator14
      _)
    (:NewEnumerator17
      _)
    (:NewEnumerator11
      _)
    (:NewEnumerator12
      _))
  (Default|SetIdle (Variables|Default|GetStateComponent)))

(event Custom|OnStateTypeChanged
  (params (InPrevType :type EStateType%20Enum :default "NewEnumerator0") (InNewType :type EStateType%20Enum :default "NewEnumerator0"))
  (Development|PrintString (Utilities|String|EnumtoString InNewType) true true "(R=1.000000,G=0.050181,B=0.020335,A=1.000000)" 5.0)
  (switch Utilities|FlowControl|Switch|SwitchonEStateType InNewType
    (:NewEnumerator5
      (CallFunction|Hitted))
    (:NewEnumerator7
      (CallFunction|BeginDead))
    (:NewEnumerator14
      (Character|LaunchCharacter (Math|Vector|MakeVector 0.0 0.0 1e+03) false false))
    (:NewEnumerator17
      (Animation|PlayAnimMontage (Variables|Hit|GetBoundUpAirAnim) 1.25 "None"))
    (:NewEnumerator11
      (Animation|PlayAnimMontage (Variables|Hit|GetBoundUpLandAnim) 1.25 "None"))
    (:NewEnumerator12
      (Animation|PlayAnimMontage (Variables|Hit|GetRiseAnim) 1.0 "None"))))

(event Custom|Hitted
  (bind _hittedordead (Hit|SetDamage))
  (if _hittedordead
    (Utilities|FlowControl|Sequence
      (:then_0
        (Hit|PlayHitAnim)
        (CallFunction|SetRotation))
      (:then_1
        (Hit|SetColor)
        (CallFunction|PlayParticle)
        (CallFunction|PlaySound)
        (Hit|PlayHitStop)
        (Hit|PlayCameraShake))
      (:then_2
        (CC|HitCC)
        (Hit|SpawnBlood))
      (:then_3
        (Hit|DropItem)))
    (else
      (Hit|SetColor)
      (CallFunction|PlayParticle)
      (CallFunction|PlaySound)
      (Hit|PlayHitStop)
      (Hit|PlayCameraShake)
      (Default|SetDead (Variables|Default|GetStateComponent)))))

(event EventDamaged
  (params (Attacker :type BP%20Character%20Object%20Reference) (Causer :type Actor%20Object%20Reference) (HitData :type F%20Hit%20Data%20Structure))
  (CallFunction|SetDamagedInfo Attacker Causer HitData))

(event EventBeginPlay
  (|CallParentFunction)
  (EventDispatchers|BindEventtoOnStateTypeChanged (Variables|Default|GetStateComponent) (EventDispatchers|CreateEvent :!event Custom|OnStateTypeChanged))
  (Utilities|FlowControl|Sequence
    (:then_0
      (Settings|SetMaterial))
    (:then_1
      (세팅|SetStatus))
    (:then_2
      (세팅|SetTargetWidget))
    (:then_3
      (세팅|SetMinimapIcon))
    (:then_4
      (CallFunction|RenderStateText))))

(event Custom|Begin_Dead
  (Animation|PlayAnimMontage (Variables|Hit|GetDeadAnim) 1.0 "None")
  (bind _asi_reward (Utilities|Casting|CastToI_Reward (Variables|Default|GetAttacker)))
  (Default|Rewarded _asi_reward self (Variables|Status|GetRewardExp)))

(event Custom|End_Dead
  (Effects|SpawnEmitteratLocation "/Game/Effects/TrailPack/Particles/Soul/Aura/P_SoulAura.P_SoulAura" (Transformation|GetActorLocation))
  (Audio|PlaySoundatLocation "/Game/Sounds/Action/Die.Die" (Transformation|GetActorLocation) "0, 0, 0" 1.0 1.0 0.0 0 0 0))