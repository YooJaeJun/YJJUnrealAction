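; BP_Character is a character Blueprint that appears to serve as a base, with empty or overridable hooks for state restore, hit end, menu events and possession.
; It reads StateComponent and MovingComponent, starting at sprint speed and matching walk speed to a speed type.
; Helpers toggle and billboard a state text, play effects and launch the character backward on hits from other groups.
; Several functions are stubs or use zeroed, self-targeting inputs.
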(fn ConstructionScript)

(fn RestoreState)

(fn RenderStateText
  (bind _statetextrender (Variables|Default|GetStateTextRender))
  (if (not (Variables|/Script/Engine.SceneComponent|GetbVisible _statetextrender))
    (Rendering|SetVisibility _statetextrender true false)))

(fn DontRenderStateText
  (bind _statetextrender (Variables|Default|GetStateTextRender))
  (if (Variables|/Script/Engine.SceneComponent|GetbVisible _statetextrender)
    (Rendering|SetVisibility _statetextrender false false)))

(fn BilboardStateText
  (bind _statetextrender (Variables|Default|GetStateTextRender))
  (Transformation|SetWorldRotation _statetextrender (Math|Rotator|MakeRotfromX (- (Transformation|GetActorLocation (Game|GetPlayerCameraManager 0)) (Transformation|GetWorldLocation _statetextrender))) false false))

(fn LaunchHit
  (Character|LaunchCharacter (* (Transformation|GetActorForwardVector) (* (.Launch (Utilities|Struct|BreakFHitData)) -1.0)) false false))

(fn SetRotation
  (Transformation|SetActorRotation (Math|Rotator|MakeRotator 0.0 0.0 (.yaw (Math|Rotator|FindLookatRotation (Transformation|GetActorLocation) (Transformation|GetActorLocation))))))

(fn PlayParticle
  (bind (_damage _attacktype _montage _playrate _canmove _launch _cc _hitstop _sound _shakeclass _effect _effectlocation _effectscale) (Utilities|Struct|BreakFHitData))
  (Effects|SpawnEmitteratLocation _effect "0, 0, 0" (Transformation|GetActorRotation) _effectscale))

(fn PlaySound
  (Audio|SpawnSoundatLocation (.Sound (Utilities|Struct|BreakFHitData)) "0, 0, 0" "0, 0, 0" 1.0 1.0 0.0 "/Game/Assets/Sounds/Weapons/SA_Sound.SA_Sound" 0))

(fn SetDamagedInfo
  (params (InAttacker :type BP%20Character%20Object%20Reference) (InCauser :type Actor%20Object%20Reference) (InHitData :type F%20Hit%20Data%20Structure) (InHitPoint :type Vector))
  (if (not (CallFunction|IsSameGroup InAttacker self))
    (Hit|LaunchHit)
    (if (Default|IsDead (Variables|Default|GetStateComponent))
      _)))

(fn LaunchBack
  (bind _returnvalue (Transformation|GetActorForwardVector))
  (bind _returnvalue_2 (* 0.0 -1.0))
  (bind _returnvalue_3 (* _returnvalue _returnvalue_2))
  (Character|LaunchCharacter (Math|Vector|MakeVector (.x _returnvalue_3) (.y _returnvalue_3) 1e+03) false false))

(fn GetCurrentSpeedType
  (bind _movingcomponent (Variables|Default|GetMovingComponent))
  (Utilities|IsValid _movingcomponent
    (:Is%20Valid
      (for (_array_element _array_index) (Variables|/Game/Components/MovingComponent.MovingComponent_C|GetSpeeds _movingcomponent)
        (if (Math|Float|NearlyEqual(Float) _array_element (Variables|/Script/Engine.CharacterMovementComponent|GetMaxWalkSpeed (Variables|Character|GetCharacterMovement)) 1.0)
          (return (Utilities|Enum|ByteToEnumESpeedType (Math|Conversions|ToByte(Integer) _array_index))))))))

(event EventUnHoveredEquipMenu
  (params (InName :type String))
  ;[1 1 1] Override
)

(event EventClickedEquipMenu
  (params (InName :type String))
  ;[1 1 1] Override
)

(event EventHoveredMagicMenu
  (params (InName :type String))
  ;[1 1 1] Override
)

(event EventUnHoveredMagicMenu
  (params (InName :type String))
  ;[1 1 1] Override
)

(event EventClickedMagicMenu
  (params (InName :type String))
  ;[1 1 1] Override
)

(event EventHoveredEquipMenu
  (params (InName :type String))
  ;[1 1 1] Override
)

(event EventTogglePossess
  (params (InEnable :type Boolean))
  (bind _returnvalue (Game|GetPlayerController 0))
  ;[1 1 1] Override
  (if InEnable
    (Pawn|Possess _returnvalue self)
    (else
      (Pawn|UnPossess _returnvalue))))

(event Input|ActionEvents|InputActionInteract
  (params (Key :type Key%20Structure))
  (:Pressed
    (Default|CallOnInteract)))

(event Custom|End_Hitted
  ;[1 1 1] Override : AI
  (if (Default|IsHitted (Variables|Default|GetStateComponent))
    (세팅|RestoreState)))

(event EventBeginPlay
  (Utilities|FlowControl|Sequence
    (:then_0
      (Variables|/Script/Engine.CharacterMovementComponent|SetMaxWalkSpeed (Variables|Character|GetCharacterMovement) (Default|GetSprintSpeed (Variables|Default|GetMovingComponent))))))

(fn GetAction
  (return ""))