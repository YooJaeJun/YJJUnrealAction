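; BP_Animal_AI is an animal AI Blueprint that extends its parent with movement speed and weapon setup at BeginPlay.
; After the parent BeginPlay, it overwrites the moving component's speed array with three tiers.
; It then spawns an actor of the weapon class at its own transform, owned by itself, and stores it as its weapon, without attaching it in this graph.
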(event EventBeginPlay
  (|CallParentFunction)
  (|SetBy-RefVar (Variables|/Game/Components/MovingComponent.MovingComponent_C|GetSpeeds (Variables|Default|GetMovingComponent)) (Utilities|Array|MakeArray 4e+02 1e+03 1.6e+03))
  (bind _returnvalue (Game|SpawnActorfromClass (Variables|Default|GetWeaponClass) (Transformation|GetActorTransform) "Undefined" self 0))
  (Variables|Default|SetWeapon _returnvalue))

(fn ConstructionScript
  (|CallParentFunction))