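; BP_Wolf is a rideable wolf that delegates its player interaction to a RidingComponent.
; An interaction collision reports overlaps to the component, and the Interact input sends it the end-interaction message to unmount.
; Action, equipment, magic, zoom and targeting inputs pass straight through, as do equip and magic menu hover and click events.
; Menu hide events share the button-release path, so the Blueprint holds no gameplay logic of its own.
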(fn ConstructionScript)

(event Input|ActionEvents|InputActionInteract
  (params (Key :type Key%20Structure :default "None"))
  (:Pressed
    (Class|IInteractable|EndInteraction(Message) (Variables|Default|GetRidingComponent))))

(event OnComponentBeginOverlap(InterationCollision)
  (params (OverlappedComponent :type Primitive%20Component%20Object%20Reference) (OtherActor :type Actor%20Object%20Reference) (OtherComp :type Primitive%20Component%20Object%20Reference) (OtherBodyIndex :type Integer) (bFromSweep :type Boolean) (SweepResult :type Hit%20Result%20Structure%20%28by%20ref%29))
  (Default|BeginOverlap (Variables|Default|GetRidingComponent) OtherActor))

(event OnComponentEndOverlap(InterationCollision)
  (params (OverlappedComponent :type Primitive%20Component%20Object%20Reference) (OtherActor :type Actor%20Object%20Reference) (OtherComp :type Primitive%20Component%20Object%20Reference) (OtherBodyIndex :type Integer))
  (Default|EndOverlap (Variables|Default|GetRidingComponent) OtherActor))

(event Input|ActionEvents|InputActionAction
  (params (Key :type Key%20Structure :default "None"))
  ;[1 1 1] Action
  (:Pressed
    (Default|Action (Variables|Default|GetRidingComponent))))

(event Input|ActionEvents|InputActionSubWeapon_Action
  (params (Key :type Key%20Structure :default "None"))
  ;[1 1 1] SubWeapon - Action
  (:Pressed
    (Default|SubWeaponActionPressed (Variables|Default|GetRidingComponent)))
  (:Released
    (Default|SubWeaponActionReleased (Variables|Default|GetRidingComponent))))

(event Input|ActionEvents|InputActionHammer
  (params (Key :type Key%20Structure :default "None"))
  (:Pressed
    (Default|Hammer (Variables|Default|GetRidingComponent))))

(event Input|ActionEvents|InputActionSword
  (params (Key :type Key%20Structure :default "None"))
  (:Pressed
    (Default|Sword (Variables|Default|GetRidingComponent))))

(event Input|ActionEvents|InputActionDual
  (params (Key :type Key%20Structure :default "None"))
  (:Pressed
    (Default|Dual (Variables|Default|GetRidingComponent))))

(event Input|ActionEvents|InputActionSubAction
  (params (Key :type Key%20Structure :default "None"))
  (:Pressed
    (Default|SubActionPressed (Variables|Default|GetRidingComponent)))
  (:Released
    (Default|SubActionReleased (Variables|Default|GetRidingComponent))))

(event Input|ActionEvents|InputActionFist
  (params (Key :type Key%20Structure :default "None"))
  (:Pressed
    (Default|Fist (Variables|Default|GetRidingComponent))))

(event Input|ActionEvents|InputActionWarp
  (params (Key :type Key%20Structure :default "None"))
  (:Pressed
    (Default|Warp (Variables|Default|GetRidingComponent))))

(event Input|ActionEvents|InputActionAround
  (params (Key :type Key%20Structure :default "None"))
  (:Pressed
    (Default|Around (Variables|Default|GetRidingComponent))))

(event Input|ActionEvents|InputActionFireBall
  (params (Key :type Key%20Structure :default "None"))
  (:Pressed
    (Default|FireBall (Variables|Default|GetRidingComponent))))

(event Input|ActionEvents|InputActionBow
  (params (Key :type Key%20Structure :default "None"))
  (:Pressed
    (Default|Bow (Variables|Default|GetRidingComponent))))

(event Input|ActionEvents|InputActionTargeting
  (params (Key :type Key%20Structure :default "None"))
  (:Pressed
    (Default|TargetingInput (Variables|Default|GetRidingComponent))))

(event Input|AxisEvents|InputAxisZoom
  (params (AxisValue :type Float%20%28single-precision%29))
  (Default|ZoomInput (Variables|Default|GetRidingComponent) AxisValue))

(event Custom|MagicMenu_Hide
  ;[1 1 1] Wrapping
  (Default|MagicMenuHide (Variables|Default|GetRidingComponent)))

(event Custom|Menu_Hide
  ;[1 1 1] Wrapping
  (Default|MenuHide (Variables|Default|GetRidingComponent)))

(event EventUnHoveredEquipMenu
  (params (InName :type String))
  ;[1 1 1] UI
  (Default|UnhoveredEquip (Variables|Default|GetRidingComponent) InName))

(event EventClickedEquipMenu
  (params (InName :type String))
  ;[1 1 1] UI
  (Default|ClickedEquip (Variables|Default|GetRidingComponent) InName))

(event EventHoveredMagicMenu
  (params (InName :type String))
  ;[1 1 1] UI
  (Default|HoveredMagic (Variables|Default|GetRidingComponent) InName))

(event EventUnHoveredMagicMenu
  (params (InName :type String))
  ;[1 1 1] UI
  (Default|UnhoveredMagic (Variables|Default|GetRidingComponent) InName))

(event EventClickedMagicMenu
  (params (InName :type String))
  ;[1 1 1] UI
  (Default|ClickedMagic (Variables|Default|GetRidingComponent) InName))

(event EventHoveredEquipMenu
  (params (InName :type String))
  ;[1 1 1] UI
  (Default|HoveredEquip (Variables|Default|GetRidingComponent) InName))

(event Input|ActionEvents|InputActionMagicMenu
  (params (Key :type Key%20Structure :default "None"))
  ;[1 1 1] Wrapping
  (:Pressed
    (Default|MagicMenu (Variables|Default|GetRidingComponent)))
  (:Released
    (Default|MagicMenuHide (Variables|Default|GetRidingComponent))))

(event Input|ActionEvents|InputActionMenu
  (params (Key :type Key%20Structure :default "None"))
  ;[1 1 1] Wrapping
  (:Pressed
    (Default|Menu (Variables|Default|GetRidingComponent)))
  (:Released
    (Default|MenuHide (Variables|Default|GetRidingComponent))))