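; Helper actor that gathers per-tick animation data for an animal Character into its Info struct.
; Tick_Info caches the owner as a Character, then derives horizontal speed, smoothed velocity-relative direction and control-rotation direction, allowing for the mesh's -90 degree yaw.
; It copies limb, pelvis and ground-slope data from an optional FeetComponent, clearing the Feet flag when that is absent or the character is falling.
; EndPlay destroys the actor.
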(event Custom|Tick_Info
  (params (InOwner :type Pawn%20Object%20Reference))
  (bind _returnvalue (Utilities|Time|GetWorldDeltaSeconds))
  (bind _info (Variables|Default|GetInfo))
  (bind _info_2 (Variables|Default|GetInfo))
  (bind _info_3 (Variables|Default|GetInfo))
  (bind _info_4 (Variables|Default|GetInfo))
  (bind _info_5 (Variables|Default|GetInfo))
  (bind _info_6 (Variables|Default|GetInfo))
  (bind _info_7 (Variables|Default|GetInfo))
  (bind _info_8 (Variables|Default|GetInfo))
  (bind _prevrotation (Utilities|Struct|BreakFAnimalAnimInfo _info_4))
  (bind _character (Utilities|Struct|BreakFAnimalAnimInfo _info_8))
  (bind _character_2 (Utilities|Struct|BreakFAnimalAnimInfo _info_2))
  (bind _character_3 (Utilities|Struct|BreakFAnimalAnimInfo _info_5))
  (bind _character_4 (Utilities|Struct|BreakFAnimalAnimInfo _info_3))
  (bind _returnvalue_2 (Actor|GetComponentbyClass _character_3 "/Game/Components/FeetComponent.FeetComponent_C"))
  (bind _returnvalue_3 (Transformation|GetVelocity _character_4))
  (bind _returnvalue_4 (Pawn|GetControlRotation _character_2 :!class /Script/Engine.Pawn))
  (bind _returnvalue_5 (Transformation|GetActorRotation _character_4))
  (bind _mesh (Variables|/Script/Engine.Character|GetMesh _character_2))
  (bind _charactermovement (Variables|/Script/Engine.Character|GetCharacterMovement _character))
  (bind _returnvalue_6 (Math|Rotator|MakeRotfromX _returnvalue_3))
  (bind _returnvalue_7 (Math|Vector|GetUpVector _mesh))
  (bind _returnvalue_8 (Math|Vector|GetForwardVector _returnvalue_4))
  (bind _returnvalue_9 (Math|Vector|GetRightVector _mesh))
  (bind _returnvalue_10 (AI|Components|NavMovement|IsFalling _charactermovement))
  (bind _returnvalue_11 (Math|Rotator|Delta(Rotator) _returnvalue_6 _returnvalue_5))
  (bind _returnvalue_12 (* _returnvalue_9 -1.0))
  (bind _returnvalue_13 (Math|Interpolation|RInterpTo _returnvalue_11 _prevrotation _returnvalue 25.0))
  (bind _returnvalue_14 (Math|Vector|CrossProduct _returnvalue_8 _returnvalue_12))
  (bind _returnvalue_15 (Math|Vector|DotProduct _returnvalue_7 _returnvalue_14))
  (Utilities|IsValid InOwner
    (:Is%20Valid
      (Utilities|IsValid (Utilities|Struct|BreakFAnimalAnimInfo (Variables|Default|GetInfo))
        (:Is%20Valid
          _)
        (:Is%20Not%20Valid
          (Utilities|IsValid InOwner
            (:Is%20Valid
              (bind _ascharacter (Utilities|Casting|CastToCharacter InOwner))
              (Utilities|Struct|SetmembersinFAnimalAnimInfo (Variables|Default|GetInfo) _ascharacter)))))
      (Utilities|FlowControl|Sequence
        (:then_0
          (Utilities|Struct|SetmembersinFAnimalAnimInfo (Variables|Default|GetInfo) (Math|Vector|VectorLengthXY _returnvalue_3))
          (Utilities|Struct|SetmembersinFAnimalAnimInfo (Variables|Default|GetInfo) _returnvalue_13)
          (Utilities|Struct|SetmembersinFAnimalAnimInfo (Variables|Default|GetInfo) (* (.Yaw (Math|Rotator|BreakRotator _returnvalue_13)) -1.0)))
        (:then_1
          (Utilities|Struct|SetmembersinFAnimalAnimInfo _info _returnvalue_15)
          (Utilities|Struct|SetmembersinFAnimalAnimInfo _info (* _returnvalue_15 1.8e+02)))
        (:then_2
          (Utilities|IsValid _returnvalue_2
            (:Is%20Valid
              (Utilities|Struct|SetmembersinFAnimalAnimInfo _info_7 (Variables|/Game/Components/FeetComponent.FeetComponent_C|GetData _returnvalue_2))
              (Utilities|Struct|SetmembersinFAnimalAnimInfo _info_7 true)
              (Utilities|Struct|SetmembersinFAnimalAnimInfo _info_6 (Variables|/Game/Components/FeetComponent.FeetComponent_C|GetLeftFoot _returnvalue_2))
              (Utilities|Struct|SetmembersinFAnimalAnimInfo _info_6 (Variables|/Game/Components/FeetComponent.FeetComponent_C|GetRightFoot _returnvalue_2))
              (Utilities|Struct|SetmembersinFAnimalAnimInfo _info_6 (Variables|/Game/Components/FeetComponent.FeetComponent_C|GetLeftHand _returnvalue_2))
              (Utilities|Struct|SetmembersinFAnimalAnimInfo _info_6 (Variables|/Game/Components/FeetComponent.FeetComponent_C|GetRightHand _returnvalue_2))
              (Utilities|Struct|SetmembersinFAnimalAnimInfo _info_6 (Variables|/Game/Components/FeetComponent.FeetComponent_C|GetPelvis _returnvalue_2))
              (Utilities|Struct|SetmembersinFAnimalAnimInfo (Variables|Default|GetInfo) (Variables|/Game/Components/FeetComponent.FeetComponent_C|GetGroundSlope _returnvalue_2)))
            (:Is%20Not%20Valid
              (Utilities|Struct|SetmembersinFAnimalAnimInfo (Variables|Default|GetInfo) false))))
        (:then_3
          (Utilities|Struct|SetmembersinFAnimalAnimInfo (Variables|Default|GetInfo) _returnvalue_10)
          (if _returnvalue_10
            (Utilities|Struct|SetmembersinFAnimalAnimInfo (Variables|Default|GetInfo) false)))))))

(event EventEndPlay
  (params (EndPlayReason :type EEndPlayReason%20Enum :default "Destroyed"))
  (Actor|DestroyActor self))

(fn ConstructionScript)