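; BP_Animal is a damageable animal character with a health bar widget, hit reactions and death.
; Damage from another group launches it and, unless dead, sets the state component to Hitted, which applies damage.
; HitData drives particles, sound, plus hit stop and camera shake for player attackers.
; Hit stop near-freezes pawns and movable-mesh actors via CustomTimeDilation; survivors turn to the attacker and bleed, others die and despawn.
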(fn ConstructionScript)

(fn PlayHitAnim
  (Components|Animation|PlayAnimation (Variables|Character|GetMesh) (Variables|Anim|GetHitAnim) false)
  (return))

(fn SetRotation
  (Transformation|SetActorRotation (Math|Rotator|MakeRotator 0.0 0.0 (.yaw (Math|Rotator|FindLookatRotation (Transformation|GetActorLocation) (Transformation|GetActorLocation (Variables|Hit|GetAttacker))))))
  (return))

(fn PlayParticle
  (bind _returnvalue (Transformation|GetActorRotation))
  (bind _hitdata (Variables|Hit|GetHitData))
  (Effects|SpawnEmitteratLocation (.effect _hitdata) (+ (Transformation|GetActorLocation) (Math|Vector|RotateVector (.effectlocation _hitdata) _returnvalue)) _returnvalue (.effectscale _hitdata))
  (return))

(fn PlaySound
  (Audio|SpawnSoundatLocation (.Sound (Utilities|Struct|BreakFHitData (Variables|Hit|GetHitData))) (Transformation|GetActorLocation) "0, 0, 0" 1.0 1.0 0.0 "/Game/Sounds/Weapons/SA_Sound.SA_Sound" 0)
  (Audio|PlaySoundatLocation "/Game/Sounds/Animals/Die_Animal.Die_Animal" (Transformation|GetActorLocation) "0, 0, 0" 1.0 1.0 0.0 0 0 0)
  (return))

(fn PlayHitStop
  (bind _returnvalue (Actor|GetComponentbyClass "/Script/Engine.MeshComponent"))
  (Utilities|Casting|CastToBP_Player (Variables|Hit|GetAttacker))
  (if (not (Math|Float|NearlyEqual(Float) (.HitStop (Utilities|Struct|BreakFHitData (Variables|Hit|GetHitData))) 0.0 1e-06))
    (bind _outactors (Actor|GetAllActorsOfClass "/Script/Engine.Actor"))
    (for _array_element _outactors
      (Utilities|Casting|CastToPawn _array_element
        (:then
          (Utilities|Array|Add (Variables|Hit|GetDilationActors) _array_element :!label _label)
          (Variables|/Script/Engine.Actor|SetCustomTimeDilation _array_element 0.001))
        (:CastFailed
          (Utilities|IsValid _returnvalue
            (:Is%20Valid
              (if (Utilities|Enum|Equal(Enum) (Variables|/Script/Engine.SceneComponent|GetMobility _returnvalue) "Movable")
                (goto _label)))))))
    (Utilities|Time|SetTimerbyFunctionName self "RestoreTimeDilation" (.HitStop (Utilities|Struct|BreakFHitData (Variables|Hit|GetHitData))))
    (return)))

(fn RestoreTimeDilation
  (bind _dilationactors (Variables|Hit|GetDilationActors))
  (for _array_element _dilationactors
    (Utilities|IsValid _array_element
      (:Is%20Valid
        (Variables|/Script/Engine.Actor|SetCustomTimeDilation _array_element 1.0))))
  (Utilities|Array|Clear _dilationactors))

(fn PlayCameraShake
  (bind _hitdata (Variables|Hit|GetHitData))
  (bind _shakeclass (Utilities|Struct|BreakFHitData _hitdata))
  (Utilities|Casting|CastToBP_Player (Variables|Hit|GetAttacker))
  (if (Utilities|IsValidClass _shakeclass)
    (CameraShakes|StartCameraShake (Game|GetPlayerCameraManager 0) _shakeclass 1.0 "CameraLocal" "0, 0, 0"))
  (return))

(fn LoadPrevState
  (if (not (Default|IsDeadMode (Variables|Default|GetStateComponent)))
    (Default|SetIdleMode (Variables|Default|GetStateComponent))
    (return)))

(fn Launch
  (Character|LaunchCharacter (* (Transformation|GetActorForwardVector) (* (.Launch (Utilities|Struct|BreakFHitData (Variables|Hit|GetHitData))) -1.0)) false false)
  (return))

(fn SetDamage
  (Variables|Status|SetHp (Math|Float|Clamp(Float) (- (Variables|Status|GetHp) (.Damage (Utilities|Struct|BreakFHitData (Variables|Hit|GetHitData)))) 0.0 (Variables|Status|GetMaxHp)))
  (Default|SetHpPercent (Variables|Status|GetHpBar_UI) (/ (Variables|Status|GetHp) (Variables|Status|GetMaxHp)))
  (return (> (Variables|Status|GetHp) 0.0)))

(fn SpawnBlood
  (Game|SpawnActorfromClass "/Game/Assets/sA_BloodSplatter_System/Blueprints/BP_Splater_Preset_2.BP_Splater_Preset_2_C" (Transformation|GetActorTransform) "Undefined" 0 0)
  (Audio|PlaySoundatLocation "/Game/Sounds/Hits/Blood_Fart_6.Blood_Fart_6" (Transformation|GetActorLocation) "0, 0, 0" 1.0 1.0 0.0 0 0 0))

(event Custom|OnStateTypeChanged
  (params (InPrevType :type EStateType%20Enum :default "NewEnumerator0") (InNewType :type EStateType%20Enum :default "NewEnumerator0"))
  (switch Utilities|FlowControl|Switch|SwitchonEStateType InNewType
    (:NewEnumerator5
      (CallFunction|Hitted))))

(event EventBeginPlay
  ;[1 1 1] 상태 타입 변경 이벤트 바인딩
  (EventDispatchers|BindEventtoOnStateTypeChanged (Variables|Default|GetStateComponent) (EventDispatchers|CreateEvent :!event Custom|OnStateTypeChanged))
  (Utilities|FlowControl|Sequence
    (:then_0
      (|SetHp))
    (:then_1
      (Rendering|SetVisibility (Variables|Default|GetHpBarWidget) false false))))

(event Custom|Hitted
  (bind _hittedordead (Hit|SetDamage))
  (if _hittedordead
    (Utilities|FlowControl|Sequence
      (:then_0
        (Hit|PlayHitAnim)
        (Hit|SetRotation))
      (:then_1
        (Hit|PlayParticle)
        (Hit|PlaySound)
        (Hit|PlayHitStop)
        (Hit|PlayCameraShake)
        (Hit|SpawnBlood)))
    (else
      (Hit|PlayParticle)
      (Hit|PlaySound)
      (Hit|PlayHitStop)
      (Hit|PlayCameraShake)
      (CallFunction|BeginDead))))

(event EventDamaged
  (params (Attacker :type Character%20Object%20Reference) (Causer :type Actor%20Object%20Reference) (HitData :type F%20Hit%20Data%20Structure))
  (if (CallFunction|CheckDifferentGroup Attacker)
    (Hit|Launch)
    (if (not (Default|IsDeadMode (Variables|Default|GetStateComponent)))
      (Variables|Hit|SetAttacker Attacker)
      (Variables|Hit|SetCauser Causer)
      (Variables|Hit|SetHitData HitData)
      (Default|SetHittedMode (Variables|Default|GetStateComponent)))))

(event Custom|End_Dead
  (Utilities|FlowControl|Delay 4.0)
  (Actor|DestroyActor))

(event Custom|Begin_Dead
  (Default|SetDeadMode (Variables|Default|GetStateComponent))
  (Components|Animation|PlayAnimation (Variables|Character|GetMesh) (Variables|Anim|GetDeadAnim) false)
  (Audio|PlaySoundatLocation "/Game/Sounds/Animals/Die_Animal.Die_Animal" (Transformation|GetActorLocation) "0, 0, 0" 1.0 1.0 0.0 0 0 0)
  (CallFunction|EndDead))