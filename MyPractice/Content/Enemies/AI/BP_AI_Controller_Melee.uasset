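; AI controller for melee enemies that runs the possessed enemy's behavior tree and picks its combat target.
; On possess, it stores the BP_Enemy_AI pawn and starts that pawn's tree.
; Each perception update scans currently perceived actors and writes the first player, or enemy with a different GroupIndex, to the blackboard's Target key.
; When no such actor is found, it clears Target.
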(event OnPerceptionUpdated(AIPerception)
  (params (UpdatedActors :type Array%20of%20Actor%20Object%20References))
  (CallFunction|Perception))

(event EventPossess
  (params (PossessedPawn :type Pawn%20Object%20Reference))
  (bind _asbp_enemy_ai (Utilities|Casting|CastToBP_Enemy_AI PossessedPawn))
  (bind _output_get (Variables|Default|SetEnemy_AI _asbp_enemy_ai))
  (AI|RunBehaviorTree (Variables|/Game/Enemies/AI/BP_Enemy_AI.BP_Enemy_AI_C|GetBehaviorTree _output_get)))

(fn ConstructionScript)

(fn Perception
  (for _array_element (Class|AIPerceptionComponent|GetCurrentlyPerceivedActors (Variables|Default|GetAIPerception))
    (bind _asbp_player (Utilities|Casting|CastToBP_Player _array_element)
      (:then
        (AI|Components|Blackboard|SetValueasObject (AI|GetBlackboard 0) (Utilities|Name|MakeLiteralName "Target") _asbp_player)
        (return))
      (:CastFailed
        (bind _asbp_enemy (Utilities|Casting|CastToBP_Enemy _array_element))
        (bind _asbp_enemy_2 (Utilities|Casting|CastToBP_Enemy (Pawn|GetControlledPawn)))
        (if (!= (.GroupIndex (Utilities|Struct|BreakFCharacterInfo (Variables|/Game/Enemies/BP_Enemy.BP_Enemy_C|GetCharacterInfo _asbp_enemy))) (.GroupIndex (Utilities|Struct|BreakFCharacterInfo (Variables|/Game/Enemies/BP_Enemy.BP_Enemy_C|GetCharacterInfo _asbp_enemy_2))))
          (AI|Components|Blackboard|SetValueasObject (AI|GetBlackboard 0) (Utilities|Name|MakeLiteralName "Target") _asbp_enemy)
          (return)))))
  (AI|Components|Blackboard|SetValueasObject (AI|GetBlackboard 0) (Utilities|Name|MakeLiteralName "Target") 0))