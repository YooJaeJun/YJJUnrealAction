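; Base or concrete AI enemy Blueprint that links combat state changes to its AI Blackboard and handles death cleanup.
; Hit, airborne-hit and knockdown states write one Behavior enum value, and the end of a hit or rise writes another.
; Getting hit also enables random-pattern action on a compatible main weapon.
; Death spawns a soul aura and sound, destroys the weapons, then removes the actor.
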(event Custom|OnStateTypeChanged_AI
  (params (InPrevType :type EStateType%20Enum :default "NewEnumerator0") (InNewType :type EStateType%20Enum :default "NewEnumerator0"))
  (switch Utilities|FlowControl|Switch|SwitchonEStateType InNewType
    (:NewEnumerator5
      _)
    (:NewEnumerator14
      _)
    (:NewEnumerator17
      _)
    (:NewEnumerator11
      _))
  (AI|Components|Blackboard|SetValueasEnum (AI|GetBlackboard (AI|GetAIController self)) (Utilities|Name|MakeLiteralName "Behavior") (Utilities|Enum|LiteralenumEBehaviorType "NewEnumerator19")))

(event EventEndDead
  (bind _weaponcomponent (Variables|Default|GetWeaponComponent))
  (bind _weaponcomponent_2 (Variables|Default|GetWeaponComponent))
  (bind _mainweapon (Variables|/Game/Components/WeaponComponent.WeaponComponent_C|GetMainWeapon _weaponcomponent))
  (bind _subweapon (Variables|/Game/Components/WeaponComponent.WeaponComponent_C|GetSubWeapon _weaponcomponent_2))
  (|CallParentFunction)
  (Effects|SpawnEmitteratLocation "/Game/Effects/P_SoulAura.P_SoulAura" (Transformation|GetActorLocation))
  (Audio|PlaySoundatLocation "/Game/Sounds/Action/Die.Die" (Transformation|GetActorLocation) "0, 0, 0" 1.0 1.0 0.0 0 0 0)
  (Utilities|IsValid _mainweapon
    (:Is%20Valid
      (Default|Destroy _mainweapon)
      (Utilities|IsValid _subweapon
        (:Is%20Valid
          (Default|Destroy _subweapon))
        (:Is%20Not%20Valid
          _)))
    (:Is%20Not%20Valid
      _))
  (Actor|DestroyActor))

(event EventHitted
  (|CallParentFunction)
  (Hit|SetEnableRandomWeaponAction))

(event EventEndHitted
  (|CallParentFunction)
  (AI|Components|Blackboard|SetValueasEnum (AI|GetBlackboard (AI|GetAIController self)) (Utilities|Name|MakeLiteralName "Behavior") (Utilities|Enum|LiteralenumEBehaviorType "NewEnumerator14")))

(event EventBeginPlay
  (|CallParentFunction)
  (EventDispatchers|BindEventtoOnStateTypeChanged (Variables|Default|GetStateComponent) (delegate Custom|OnStateTypeChanged_AI)))

(event EventEndRise
  (|CallParentFunction)
  (AI|Components|Blackboard|SetValueasEnum (AI|GetBlackboard (AI|GetAIController self)) (Utilities|Name|MakeLiteralName "Behavior") (Utilities|Enum|LiteralenumEBehaviorType "NewEnumerator14")))

(fn ConstructionScript
  (|CallParentFunction))

(fn SetEnableRandomWeaponAction
  (bind _asweapon_random_pattern (Utilities|Casting|CastToWeapon_RandomPattern (Variables|/Game/Components/WeaponComponent.WeaponComponent_C|GetMainWeapon (Variables|Default|GetWeaponComponent))))
  (Variables|/Game/Weapons/Weapon_RandomPattern.Weapon_RandomPattern_C|SetEnable _asweapon_random_pattern true)
  (return))