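; BP_Bloodstain_Main is a bloodstain decal actor that animates in, lingers, then dissolves and destroys itself.
; Shortly after BeginPlay, it takes the Plane's material, creates a dynamic instance and assigns it to the Decal, so the Plane supplies the stain's look.
; One timeline drives the Opening_Rate parameter, then after a Lifetime delay the Dissolving timeline drives the "qq" parameter before the actor is destroyed.
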(event EventBeginPlay
  (bind _plane (Variables|Default|GetPlane))
  (bind _decal (Variables|Default|GetDecal))
  (bind _returnvalue (Rendering|Material|GetMaterial _plane 0))
  (Utilities|FlowControl|Delay 0.1)
  (Utilities|IsValid _plane
    (:Is%20Valid
      (Utilities|IsValid _returnvalue
        (:Is%20Valid
          (Variables|Default|SetStatic_Material _returnvalue)
          (Utilities|IsValid _decal
            (:Is%20Valid
              (Rendering|Components|Decal|SetDecalMaterial _decal _returnvalue)
              (Utilities|IsValid (Variables|Default|GetStatic_Material)
                (:Is%20Valid
                  (bind _returnvalue_2 (Rendering|Material|CreateDynamicMaterialInstance (Variables|Default|GetPlane) 0 (Variables|Default|GetStatic_Material) "None" :!class /Script/Engine.PrimitiveComponent))
                  (Utilities|IsValid _returnvalue_2
                    (:Is%20Valid
                      (bind _output_get (Variables|Default|SetMaterial _returnvalue_2))
                      (Rendering|Components|Decal|SetDecalMaterial (Variables|Default|GetDecal) _output_get)
                      (bind _dissolve_rate (Timeline|Timeline_0 Play)
                        (:Update
                          (Rendering|Material|SetScalarParameterValue _output_get "Opening_Rate" _dissolve_rate :!class /Script/Engine.MaterialInstanceDynamic))
                        (:Finished
                          (Utilities|FlowControl|Delay (Variables|Default|GetLifetime))
                          (bind _dissolve_rate_2 (Timeline|Dissolving Play)
                            (:Update
                              (Rendering|Material|SetScalarParameterValue _output_get "qq" _dissolve_rate_2 :!class /Script/Engine.MaterialInstanceDynamic))
                            (:Finished
                              (Actor|DestroyActor))))))))))))))))

(fn ConstructionScript)