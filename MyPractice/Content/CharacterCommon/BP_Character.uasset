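; BP_Character is a common character Blueprint providing hit recovery, interaction, footstep audio and group checks.
; When a hit ends, it uses the StateComponent's previous state to return to idle, falling or riding.
; The Interact input messages a registered interactable once, while ToggleInput possesses or unpossesses the character.
; It also swaps animation Blueprints and plays footstep sounds by surface type, defaulting to grass.
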(fn ConstructionScript)

(fn CheckDifferentGroup
  (params (Character :type Actor%20Object%20Reference))
  (bind _asbp_character (Utilities|Casting|CastToBP_Character Character)
    (:then
      (return (!= (.GroupIndex (Utilities|Struct|BreakFCharacterInfo (Variables|BP_Character_C|GetCharacterInfo _asbp_character))) (.GroupIndex (Utilities|Struct|BreakFCharacterInfo (Variables|Default|GetCharacterInfo self))))))
    (:CastFailed
      (return true))))

(event Custom|End_Hitted
  (bind _returnvalue (Actor|GetComponentbyClass "/Game/Components/StateComponent.StateComponent_C"))
  ;[1 1 1] Override
  (switch Utilities|FlowControl|Switch|SwitchonEStateType (Variables|/Game/Components/StateComponent.StateComponent_C|GetPrevType _returnvalue)
    (:NewEnumerator0
      (Default|SetIdleMode _returnvalue :!label _label))
    (:NewEnumerator2
      (goto _label))
    (:NewEnumerator3
      (goto _label))
    (:NewEnumerator4
      (goto _label))
    (:NewEnumerator5
      (goto _label))
    (:NewEnumerator6
      (goto _label))
    (:NewEnumerator10
      (Default|SetFallingMode _returnvalue :!label _label_2))
    (:NewEnumerator13
      (goto _label_2))
    (:NewEnumerator14
      (goto _label_2))
    (:NewEnumerator17
      (goto _label_2))
    (:NewEnumerator11
      (goto _label_2))
    (:NewEnumerator12
      (goto _label))
    (:NewEnumerator19
      (Default|SetRidingMode _returnvalue))))

(event EventRegisterInteractableActor
  (params (InteractableActor :type Actor%20Object%20Reference))
  ;[1 1 1] Override
  (Variables|Default|SetInteractableActor InteractableActor))

(event EventChangeAnimationBlueprint
  (params (InABPClass :type Object%20Class%20Reference))
  (Class|SkeletalMeshComponent|SetAnimClass (Variables|Character|GetMesh) InABPClass))

(event EventToggleInput
  (params (InEnable :type Boolean))
  (bind _returnvalue (Game|GetPlayerController 0))
  ;[1 1 1] Override
  (if InEnable
    (Pawn|Possess _returnvalue self)
    (else
      (Pawn|UnPossess _returnvalue))))

(event Input|ActionEvents|InputActionInteract
  (params (Key :type Key%20Structure :default "None"))
  (:Pressed
    (Utilities|IsValid (Variables|Default|GetInteractableActor)
      (:Is%20Valid
        (Class|IInteractable|StartInteraction(Message) (Variables|Default|GetInteractableActor) self)
        (Variables|Default|SetInteractableActor 0)))))

(event EventFootstep
  (params (Left_or_Right :type Boolean) (SurfaceType :type EPhysicalSurface%20Enum :default "SurfaceType_Default") (StepLocation :type Vector :default "0, 0, 0"))
  (switch Utilities|FlowControl|Switch|SwitchonEPhysicalSurface SurfaceType
    (:SurfaceType_Default
      (Audio|PlaySoundatLocation "/Game/Sounds/Footsteps/Jog/Grass/SC_Footstep_Grass_Jog.SC_Footstep_Grass_Jog" StepLocation "0, 0, 0" 1.0 1.0 0.0 0 0 0 :!label _label))
    (:SurfaceType1
      (goto _label))
    (:SurfaceType2
      (Audio|PlaySoundatLocation "/Game/Sounds/Footsteps/Jog/Wood/SC_Footstep_Wood_Jog.SC_Footstep_Wood_Jog" StepLocation "0, 0, 0" 1.0 1.0 0.0 0 0 0))
    (:SurfaceType3
      (Audio|PlaySoundatLocation "/Game/Sounds/Footsteps/Jog/Sand/SC_Footstep_Sand_Jog.SC_Footstep_Sand_Jog" StepLocation "0, 0, 0" 1.0 1.0 0.0 0 0 0))
    (:SurfaceType4
      (Audio|PlaySoundatLocation "/Game/Sounds/Footsteps/Jog/Stone/SC_Footstep_Stone_Jog.SC_Footstep_Stone_Jog" StepLocation "0, 0, 0" 1.0 1.0 0.0 0 0 0))
    (:SurfaceType5
      (Audio|PlaySoundatLocation "/Game/Sounds/Footsteps/Jog/Splash/SC_Footstep_Splash_Jog.SC_Footstep_Splash_Jog" StepLocation "0, 0, 0" 1.0 1.0 0.0 0 0 0))))

(fn IsPlayer
  (return (Pawn|IsPlayerControlled)))