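; BP_Character is a character Blueprint with hit recovery, riding interaction and group-based differentiation between characters.
; When a hit ends, End_Hitted uses the StateComponent's previous state to choose idle, riding or falling mode.
; Interact input starts riding through the registered actor's RidingComponent, while helpers toggle possession and swap the animation Blueprint.
; CheckDifferentGroup compares group indices, treating non-BP_Character targets as different, and equip/magic menu events are empty stubs.
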(fn ConstructionScript)

(fn CheckDifferentGroup
  (params (Character :type Actor%20Object%20Reference))
  (bind _asbp_character (Utilities|Casting|CastToBP_Character Character)
    (:then
      (return (!= (.GroupIndex (Utilities|Struct|BreakFCharacterInfo (Variables|BP_Character_C|GetCharacterInfo _asbp_character))) (.GroupIndex (Utilities|Struct|BreakFCharacterInfo (Variables|Default|GetCharacterInfo self))))))
    (:CastFailed
      (return true))))

(event Custom|End_Hitted
  (bind _returnvalue (Actor|GetComponentbyClass "/Game/Components/StateComponent.StateComponent_C"))
  ;[1 1 1] Override : AI
  (switch Utilities|FlowControl|Switch|SwitchonEStateType (Variables|/Game/Components/StateComponent.StateComponent_C|GetPrevType _returnvalue)
    (:NewEnumerator0
      (Default|SetIdleMode _returnvalue :!label _label))
    (:NewEnumerator2
      (goto _label))
    (:NewEnumerator3
      (Utilities|IsValid (Variables|Default|GetCurRiddenActor) :!label _label_2
        (:Is%20Valid
          (Default|SetRidingMode _returnvalue))
        (:Is%20Not%20Valid
          (Default|SetIdleMode _returnvalue))))
    (:NewEnumerator4
      (goto _label_2))
    (:NewEnumerator5
      (goto _label_2))
    (:NewEnumerator6
      (Default|SetFallingMode _returnvalue :!label _label_3))
    (:NewEnumerator10
      (goto _label_3))
    (:NewEnumerator13
      (goto _label_3))
    (:NewEnumerator14
      (goto _label_3))
    (:NewEnumerator17
      (goto _label_3))
    (:NewEnumerator11
      (goto _label_3))
    (:NewEnumerator12
      (goto _label))
    (:NewEnumerator19
      (Default|SetRidingMode _returnvalue))))

(event EventUnHoveredEquipMenu
  (params (InName :type String))
  ;[1 1 1] Override
)

(event EventClickedEquipMenu
  (params (InName :type String))
  ;[1 1 1] Override
)

(event EventHoveredMagicMenu
  (params (InName :type String))
  ;[1 1 1] Override
)

(event EventUnHoveredMagicMenu
  (params (InName :type String))
  ;[1 1 1] Override
)

(event EventClickedMagicMenu
  (params (InName :type String))
  ;[1 1 1] Override
)

(event EventHoveredEquipMenu
  (params (InName :type String))
  ;[1 1 1] Override
)

(event EventRegisterInteractableActor
  (params (InteractableActor :type Actor%20Object%20Reference))
  ;[1 1 1] Override
  (Variables|Default|SetInteractableActor InteractableActor))

(event EventChangeAnimationBlueprint
  (params (InABPClass :type Object%20Class%20Reference))
  (Class|SkeletalMeshComponent|SetAnimClass (Variables|Character|GetMesh) InABPClass))

(event EventToggleInput
  (params (InEnable :type Boolean))
  (bind _returnvalue (Game|GetPlayerController 0))
  (bind _self self)
  ;[1 1 1] Override
  (if InEnable
    (Pawn|Possess _returnvalue self)
    (Variables|BP_Character_C|SetCurController _self (Pawn|GetController _self))
    (else
      (Pawn|UnPossess _returnvalue))))

(event Input|ActionEvents|InputActionInteract
  (params (Key :type Key%20Structure :default "None"))
  (:Pressed
    (Utilities|IsValid (Variables|Default|GetInteractableActor)
      (:Is%20Valid
        (Utilities|IsValid (Actor|GetComponentbyClass (Variables|Default|GetInteractableActor) "/Game/Components/RidingComponent.RidingComponent_C")
          (:Is%20Valid
            (Class|IInteractable|StartInteraction(Message) (Actor|GetComponentbyClass (Variables|Default|GetInteractableActor) "/Game/Components/RidingComponent.RidingComponent_C") self)
            (Variables|Default|SetInteractableActor 0)))))))

(fn IsPlayer
  (return (Pawn|IsPlayerControlled)))